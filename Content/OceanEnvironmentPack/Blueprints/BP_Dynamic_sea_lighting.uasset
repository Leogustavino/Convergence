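; Underwater lighting actor that darkens fog, skylight and sun as the player camera descends from shallow to deep sea.
; Each Tick turns camera Z into a clamped depth alpha that lerps fog and light settings, fades the caustics light function and drives the OceanGlow collection parameter.
; The construction script assigns the dynamic caustics material to the sun, sets fog height and previews a chosen depth, with optional fog hiding until BeginPlay.
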(event EventBeginPlay
  ;[1 1 1] Preview_fogdisable active only in ediotor mode
  (Rendering|SetVisibility (Variables|Default|GetExponentialHeightFog) true false))

(event EventTick
  (params (DeltaSeconds :type Float%20%28single-precision%29))
  (bind _returnvalue (Game|GetPlayerCameraManager 0))
  (bind _shallow_z_value (Variables|Fog|GetShallow_Z_value))
  (bind _deepsea_z_value (Variables|Fog|GetDeepSea_Z_Value))
  (bind _shallow_z_value_2 (Variables|Fog|GetShallow_Z_value))
  (bind _returnvalue_2 (Camera|GetCameraLocation _returnvalue))
  (bind _returnvalue_3 (Math|Float|Absolute(Float) _deepsea_z_value))
  (bind _z (Math|Vector|BreakVector _returnvalue_2))
  (bind _returnvalue_4 (+ _returnvalue_3 _shallow_z_value))
  (bind _returnvalue_5 (- _z _shallow_z_value_2))
  (bind _returnvalue_6 (/ _returnvalue_5 _returnvalue_4))
  (bind _returnvalue_7 (* _returnvalue_6 -1.0))
  (bind _returnvalue_8 (Math|Float|Clamp(Float) _returnvalue_7))
  ;[1 1 1] Darkern all color and intensity as player goes deeper
  (Class|ExponentialHeightFogComponent|SetFogInscatteringColor (Variables|Default|GetExponentialHeightFog) (Math|Color|Lerp(LinearColor) (Variables|Shallow|GetFog_Shallow) (Variables|Deep|GetFog_Deep) _returnvalue_8))
  (Class|ExponentialHeightFogComponent|SetDirectionalInscatteringColor (Variables|Default|GetExponentialHeightFog) (Math|Color|Lerp(LinearColor) (Variables|Shallow|GetFog_DirScatter_Shallow) (Variables|Deep|GetFog_DirScatter_Deep) _returnvalue_8))
  (Rendering|Components|Light|SetIntensity (Variables|Default|GetSkyLight) (Math|Float|Lerp (Variables|Shallow|GetSkylight_Intensity_shallow) (Variables|Deep|GetSkylight_Intensity_Deep) _returnvalue_8))
  (Rendering|Components|Light|SetIntensity (Variables|Default|GetDirectionalLight) (Math|Float|Lerp (Variables|Shallow|GetSun_Intensity_Shallow) (Variables|Deep|GetSun_Intensity_Deep) _returnvalue_8))
  (Rendering|Material|SetScalarParameterValue (Variables|Default|GetLightMaterial) "Multiply" (Math|Float|Lerp 1.5 -0.25 _returnvalue_8) :!class /Script/Engine.MaterialInstanceDynamic)
  (Class|ExponentialHeightFogComponent|SetFogDensity (Variables|Default|GetExponentialHeightFog) (Math|Float|Lerp (Variables|Shallow|GetFog_Density_Shallow) (Variables|Deep|GetFog_Density_Deep) _returnvalue_8))
  (Class|ExponentialHeightFogComponent|SetFogMaxOpacity (Variables|Default|GetExponentialHeightFog) (Math|Float|Lerp (Variables|Shallow|GetFog_Max_Opacity_Shallow) (Variables|Deep|GetFog_Max_Opacity_Deep) _returnvalue_8))
  (Rendering|Material|SetScalarParameterValue "/Game/OceanEnvironmentPack/Materials/ParentMaterials/MPC_OceanEnvironmentPack.MPC_OceanEnvironmentPack" "OceanGlow" _returnvalue_8 :!class /Script/Engine.KismetMaterialLibrary))

(fn ConstructionScript
  (bind _exponentialheightfog (Variables|Default|GetExponentialHeightFog))
  (bind _exponentialheightfog_2 (Variables|Default|GetExponentialHeightFog))
  (bind _previewdepth (Variables|Fog|GetPreviewDepth))
  (bind _returnvalue (Transformation|GetWorldLocation _exponentialheightfog))
  (bind (_x _y) (Math|Vector|BreakVector _returnvalue))
  ;[1 1 1] Dynamic Material Instance
  (bind _returnvalue_2 (Rendering|Material|CreateDynamicMaterialInstance "/Game/OceanFloor/Materials/M_Caustics02.M_Caustics02" "None" :!class /Script/Engine.KismetMaterialLibrary))
  (bind _output_get (Variables|Default|SetLightMaterial _returnvalue_2))
  (Rendering|Components|Light|SetLightFunctionMaterial (Variables|Default|GetDirectionalLight) _output_get)
  (Transformation|SetWorldLocation _exponentialheightfog (Math|Vector|MakeVector _x _y (Variables|Fog|GetFog_Height)) false false)
  (Class|ExponentialHeightFogComponent|SetFogInscatteringColor (Variables|Default|GetExponentialHeightFog) (Math|Color|Lerp(LinearColor) (Variables|Shallow|GetFog_Shallow) (Variables|Deep|GetFog_Deep) _previewdepth))
  (Class|ExponentialHeightFogComponent|SetDirectionalInscatteringColor (Variables|Default|GetExponentialHeightFog) (Math|Color|Lerp(LinearColor) (Variables|Shallow|GetFog_DirScatter_Shallow) (Variables|Deep|GetFog_DirScatter_Deep) _previewdepth))
  (Rendering|Components|Light|SetIntensity (Variables|Default|GetSkyLight) (Math|Float|Lerp (Variables|Shallow|GetSkylight_Intensity_shallow) (Variables|Deep|GetSkylight_Intensity_Deep) _previewdepth))
  (Rendering|Components|Light|SetIntensity (Variables|Default|GetDirectionalLight) (Math|Float|Lerp (Variables|Shallow|GetSun_Intensity_Shallow) (Variables|Deep|GetSun_Intensity_Deep) _previewdepth))
  (Class|ExponentialHeightFogComponent|SetFogDensity (Variables|Default|GetExponentialHeightFog) (Math|Float|Lerp (Variables|Shallow|GetFog_Density_Shallow) (Variables|Deep|GetFog_Density_Deep) _previewdepth))
  (Class|ExponentialHeightFogComponent|SetFogMaxOpacity (Variables|Default|GetExponentialHeightFog) (Math|Float|Lerp (Variables|Shallow|GetFog_Max_Opacity_Shallow) (Variables|Deep|GetFog_Max_Opacity_Deep) _previewdepth))
  (if (Variables|Fog|GetPreview_FogDisabled)
    (Rendering|SetVisibility _exponentialheightfog_2 false false)
    (else
      (Rendering|SetVisibility _exponentialheightfog_2 true false))))