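; BP_SphinxHead is an interactable Sphinx head monument, built as a thin child Blueprint that relies on its parent for behavior.
; Its BoxCollision overlap events forward the other actor to BeginOverlap and EndOverlap.
; Interact passes straight to the parent, while PlayerInteraction calls the parent with a fixed Monument enum value identifying this piece.
; Tick and the construction script only call their parent versions.
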(event OnComponentBeginOverlap(BoxCollision)
  (params (OverlappedComponent :type Primitive%20Component%20Object%20Reference) (OtherActor :type Actor%20Object%20Reference) (OtherComp :type Primitive%20Component%20Object%20Reference) (OtherBodyIndex :type Integer) (bFromSweep :type Boolean) (SweepResult :type Hit%20Result%20Structure%20%28by%20ref%29))
  (CallFunction|BeginOverlap OtherActor))

(event OnComponentEndOverlap(BoxCollision)
  (params (OverlappedComponent :type Primitive%20Component%20Object%20Reference) (OtherActor :type Actor%20Object%20Reference) (OtherComp :type Primitive%20Component%20Object%20Reference) (OtherBodyIndex :type Integer))
  (CallFunction|EndOverlap OtherActor))

(event EventBeginPlay
  (|CallParentFunction) ; This node is disabled and will not be called.\nDrag off pins to build functionality.
)

(event Collision|EventActorBeginOverlap
  (params (OtherActor :type Actor%20Object%20Reference))
  (|CallParentFunction OtherActor) ; This node is disabled and will not be called.\nDrag off pins to build functionality.
)

(event EventTick
  (params (DeltaSeconds :type Float%20%28single-precision%29))
  (|CallParentFunction DeltaSeconds))

(event EventInteract
  (params (PlayerInteracted :type Actor%20Object%20Reference))
  (|CallParentFunction PlayerInteracted))

(event EventPlayerInteraction
  (params (PlayerInteracted :type Actor%20Object%20Reference) (Monument :type InteractableObjects_Enum%20Enum :default "NewEnumerator8"))
  (|CallParentFunction PlayerInteracted "NewEnumerator5"))

(fn ConstructionScript
  (|CallParentFunction))