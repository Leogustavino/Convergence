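; BP_InteractionTest is a test interactable that toggles a dialogue widget on screen.
; Its Interact event removes and clears the stored widget if one is valid.
; Otherwise it creates one for player controller 0, stores it, adds it to the viewport and then sets its DialogueText from the MyText variable.
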(event EventInteract
  (params (PlayerInteracted :type Actor%20Object%20Reference))
  (Utilities|IsValid (Variables|Default|GetDialogueWidget)
    (:Is%20Valid
      (Widget|RemovefromParent (Variables|Default|GetDialogueWidget))
      (Variables|Default|SetDialogueWidget 0))
    (:Is%20Not%20Valid
      (bind _returnvalue (UserInterface|CreateWidget "/Game/_ConvergencePoint/Widgets/DialogueWidget.DialogueWidget_C" (Game|GetPlayerController 0)))
      (bind _output_get (Variables|Default|SetDialogueWidget _returnvalue))
      (UserInterface|Viewport|AddtoViewport _output_get 0)
      (Variables|/Game/_ConvergencePoint/Widgets/DialogueWidget.DialogueWidget_C|SetDialogueText (Variables|Default|GetDialogueWidget) (Variables|Default|GetMy%20Text)))))

(fn ConstructionScript)