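; A dialogue trigger volume outside the train that advances the fifth story beat to its B progression.
; When the player overlaps its box, it checks through the game manager that the dialogue beat ID is five and the monument scan count is six.
; If both hold, it calls the fifth-beat B progression and destroys itself, so it fires only once.
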(event OnComponentBeginOverlap(Box)
  (params (OverlappedComponent :type Primitive%20Component%20Object%20Reference) (OtherActor :type Actor%20Object%20Reference) (OtherComp :type Primitive%20Component%20Object%20Reference) (OtherBodyIndex :type Integer) (bFromSweep :type Boolean) (SweepResult :type Hit%20Result%20Structure%20%28by%20ref%29))
  (bind _my_game_manager (CallFunction|GetMyGameManager))
  (if (== OtherActor (Variables|/Game/_ConvergencePoint/Blueprints/MyGameManager.MyGameManager_C|GetMyPlayer _my_game_manager))
    (if (and (== (Variables|/Game/_ConvergencePoint/Blueprints/BP_Dialogue.BP_Dialogue_C|GetBeat_ID (Variables|/Game/_ConvergencePoint/Blueprints/MyGameManager.MyGameManager_C|GetDialogueBP _my_game_manager)) 5) (== (Variables|/Game/_ConvergencePoint/Blueprints/New/ObjectManager.ObjectManager_C|GetMonumentScanCount (Variables|/Game/_ConvergencePoint/Blueprints/MyGameManager.MyGameManager_C|GetObjectManager _my_game_manager)) 6))
      (Default|Call5thBeatBProgression)
      (Actor|DestroyActor))))

(fn ConstructionScript
  (|CallParentFunction))