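; BP_NewArea is a box trigger that advances story beats and announces a new area when the player enters it.
; Overlap is gated on the dialogue BeatID matching BeatDependency, then fires delayed progression calls for the second or fourth beat.
; A delayed HUD sequence shows scan progress and feedback text, then destroys the trigger.
; The second beat also registers the "area2"-tagged trigger as the game manager's NewArea.
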(event OnComponentBeginOverlap(Box)
  (params (OverlappedComponent :type Primitive%20Component%20Object%20Reference) (OtherActor :type Actor%20Object%20Reference) (OtherComp :type Primitive%20Component%20Object%20Reference) (OtherBodyIndex :type Integer) (bFromSweep :type Boolean) (SweepResult :type Hit%20Result%20Structure%20%28by%20ref%29))
  (bind _my_game_manager (CallFunction|GetMyGameManager))
  (if (== (Variables|/Game/_ConvergencePoint/Blueprints/BP_Dialogue.BP_Dialogue_C|GetBeat_ID (Variables|/Game/_ConvergencePoint/Blueprints/MyGameManager.MyGameManager_C|GetDialogueBP _my_game_manager)) (Variables|Default|GetBeatDependency))
    (if (== (Variables|/Game/_ConvergencePoint/Blueprints/MyGameManager.MyGameManager_C|GetMyPlayer _my_game_manager) OtherActor)
      (if (not (Variables|Default|GethasEnteredNewArea?))
        (Utilities|FlowControl|Sequence
          (:then_0
            (CallFunction|TriggerBeat))
          (:then_1
            (CallFunction|NewAreaText (Variables|/Game/_ConvergencePoint/Blueprints/BP_Dialogue.BP_Dialogue_C|GetBeat_ID (Variables|/Game/_ConvergencePoint/Blueprints/MyGameManager.MyGameManager_C|GetDialogueBP _my_game_manager)))))))))

(event Custom|TriggerBeat
  (bind _my_game_manager (CallFunction|GetMyGameManager))
  (if (== (Variables|/Game/_ConvergencePoint/Blueprints/BP_Dialogue.BP_Dialogue_C|GetBeat_ID (Variables|/Game/_ConvergencePoint/Blueprints/MyGameManager.MyGameManager_C|GetDialogueBP _my_game_manager)) 2)
    (Utilities|FlowControl|Delay 0.5)
    (Default|CallSecondBeatProgression)
    (elif (== (Variables|/Game/_ConvergencePoint/Blueprints/BP_Dialogue.BP_Dialogue_C|GetBeat_ID (Variables|/Game/_ConvergencePoint/Blueprints/MyGameManager.MyGameManager_C|GetDialogueBP _my_game_manager)) 4)
      (Utilities|FlowControl|Delay 0.5)
      (Default|CallFourthBBeatProgression))))

(event Custom|NewAreaText
  (params (Beat :type Integer))
  (if (== Beat 2)
    (Utilities|FlowControl|Delay 4.4)
    (CallFunction|DisplayWidget)
    (bind _outactors (Actor|GetAllActorsOfClasswithTag "BP_NewArea_C" "area2"))
    (bind _asbp_new_area (Utilities|Casting|CastToBP_NewArea (Utilities|Array|Get(acopy) _outactors)))
    (bind _my_game_manager (CallFunction|GetMyGameManager))
    (Variables|/Game/_ConvergencePoint/Blueprints/MyGameManager.MyGameManager_C|SetNewArea _my_game_manager _asbp_new_area)
    (elif (== Beat 4)
      (Utilities|FlowControl|Delay 4.6)
      (CallFunction|DisplayWidget))))

(event Custom|DisplayWidget
  (bind _my_game_manager (CallFunction|GetMyGameManager))
  (Default|EnableVisibilityScanProgress (Variables|/Game/_ConvergencePoint/Blueprints/MyGameManager.MyGameManager_C|GetHUD _my_game_manager))
  (Variables|/Game/_ConvergencePoint/Widgets/MainWidgets/HUD.HUD_C|SetFeedbackText (Variables|/Game/_ConvergencePoint/Blueprints/MyGameManager.MyGameManager_C|GetHUD _my_game_manager) "Entered a new area")
  (Utilities|FlowControl|Delay 1.5)
  (Variables|/Game/_ConvergencePoint/Widgets/MainWidgets/HUD.HUD_C|SetFeedbackText (Variables|/Game/_ConvergencePoint/Blueprints/MyGameManager.MyGameManager_C|GetHUD _my_game_manager) "3 items to scan")
  (Utilities|FlowControl|Delay 1.5)
  (Variables|/Game/_ConvergencePoint/Widgets/MainWidgets/HUD.HUD_C|SetFeedbackText (Variables|/Game/_ConvergencePoint/Blueprints/MyGameManager.MyGameManager_C|GetHUD _my_game_manager) "")
  (Variables|Default|SethasEnteredNewArea? true)
  (Actor|DestroyActor))

(fn ConstructionScript
  (Transformation|SetWorldScale3D (Variables|Default|GetBox) (Variables|Default|GetBoxCollisionScale)))

(fn UpdateCount)