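; A Blueprint function library of shared gameplay and UI helpers, built around a game manager held by MyGameMode.
; UI helpers toggle the mouse cursor with its matching input mode, create widgets hidden in the viewport, and hide all user widgets.
; Gameplay helpers test whether a given player overlaps a box and set the manager's ObjectSelection from the interactable's landmark tag (StatueOfLiberty, Maoi, Sphinx, or a fallback).
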(fn ShowMouse
  (params (Visible :type Boolean))
  (bind _returnvalue (Game|GetPlayerController 0))
  (bind _output_get (Variables|/Script/Engine.PlayerController|SetbShowMouseCursor _returnvalue Visible))
  (if _output_get
    (Input|SetInputModeGameandUI _returnvalue 0 "LockInFullscreen" false)
    (else
      (Input|SetInputModeGameOnly _returnvalue))))

(fn GetMyGameManager
  (bind _asmy_game_mode (Utilities|Casting|CastToMyGameMode (Game|GetGameMode)))
  (return (Variables|/Game/_ConvergencePoint/Blueprints/MyGameMode.MyGameMode_C|GetMy%20Game%20Manager _asmy_game_mode)))

(fn IsOverlapping
  (params (BoxCollision :type Primitive%20Component%20Object%20Reference) (PlayerInteracted :type Object%20Object%20Reference))
  (bind _array_element (Utilities|Array|ForEachLoopwithBreak (Collision|GetOverlappingActors BoxCollision "/Game/FirstPersonBP/Blueprints/FirstPersonCharacter.FirstPersonCharacter_C" :!class /Script/Engine.PrimitiveComponent) :!label _label)
    (:LoopBody
      (if (== _array_element PlayerInteracted)
        (goto _label Break)))
    (:Completed
      (return (== _array_element PlayerInteracted)))))

(fn InitWidget
  (params (ClassWidget :type User%20Widget%20Class%20Reference))
  (bind _returnvalue (UserInterface|CreateWidget ClassWidget))
  (UserInterface|Viewport|AddtoViewport _returnvalue 0)
  (Widget|SetVisibility _returnvalue "Hidden")
  (return _returnvalue))

(fn SetObjectSelection
  (bind _my_game_manager (CallFunction|GetMyGameManager))
  (if (Actor|ActorHasTag (Variables|/Game/_ConvergencePoint/Blueprints/MyGameManager.MyGameManager_C|GetInteractableObject _my_game_manager) "StatueOfLiberty")
    (Variables|/Game/_ConvergencePoint/Blueprints/MyGameManager.MyGameManager_C|SetObjectSelection _my_game_manager "NewEnumerator0")
    (elif (Actor|ActorHasTag (Variables|/Game/_ConvergencePoint/Blueprints/MyGameManager.MyGameManager_C|GetInteractableObject _my_game_manager) "Maoi")
      (Variables|/Game/_ConvergencePoint/Blueprints/MyGameManager.MyGameManager_C|SetObjectSelection _my_game_manager "NewEnumerator1")
      (elif (Actor|ActorHasTag (Variables|/Game/_ConvergencePoint/Blueprints/MyGameManager.MyGameManager_C|GetInteractableObject _my_game_manager) "Sphinx")
        (Variables|/Game/_ConvergencePoint/Blueprints/MyGameManager.MyGameManager_C|SetObjectSelection _my_game_manager "NewEnumerator2")
        (else
          (Variables|/Game/_ConvergencePoint/Blueprints/MyGameManager.MyGameManager_C|SetObjectSelection _my_game_manager "NewEnumerator5"))))))

(fn HideUI
  (bind _foundwidgets (Widget|GetAllWidgetsOfClass 0 "/Script/UMG.UserWidget" false))
  (for _array_element _foundwidgets
    (Widget|SetVisibility _array_element "Hidden")))