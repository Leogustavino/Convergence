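; Test Blueprint for an interactable statue that opens a dialog and plays an audio cue for the player.
; Its collision box toggles the game manager's interaction prompt as the player enters and leaves.
; Interact checks overlap, then a FlipFlop with only A wired removes the prompt, shows the dialog and plays audio on alternate calls.
; Tick moves the audio to the player's mesh transform every frame.
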(event OnComponentBeginOverlap(StatueCollision)
  (params (OverlappedComponent :type Primitive%20Component%20Object%20Reference) (OtherActor :type Actor%20Object%20Reference) (OtherComp :type Primitive%20Component%20Object%20Reference) (OtherBodyIndex :type Integer) (bFromSweep :type Boolean) (SweepResult :type Hit%20Result%20Structure%20%28by%20ref%29))
  ;[1 1 1] Show Interaction
  (bind _my_game_manager (CallFunction|GetMyGameManager))
  (if (== OtherActor (Variables|/Game/_ConvergencePoint/Blueprints/MyGameManager.MyGameManager_C|GetMyPlayer _my_game_manager))
    (Widget|SetVisibility (Variables|/Game/_ConvergencePoint/Blueprints/MyGameManager.MyGameManager_C|GetInteractionWidget _my_game_manager) "Visible")))

(event OnComponentEndOverlap(StatueCollision)
  (params (OverlappedComponent :type Primitive%20Component%20Object%20Reference) (OtherActor :type Actor%20Object%20Reference) (OtherComp :type Primitive%20Component%20Object%20Reference) (OtherBodyIndex :type Integer))
  ;[1 1 1] Hide Interaction
  (bind _my_game_manager (CallFunction|GetMyGameManager))
  (if (== OtherActor (Variables|/Game/_ConvergencePoint/Blueprints/MyGameManager.MyGameManager_C|GetMyPlayer _my_game_manager))
    (Widget|SetVisibility (Variables|/Game/_ConvergencePoint/Blueprints/MyGameManager.MyGameManager_C|GetInteractionWidget _my_game_manager) "Hidden")))

(event EventBeginPlay
  (Variables|Default|SetAudioCue (Variables|Default|GetFire01_Cue)))

(event Collision|EventActorBeginOverlap
  (params (OtherActor :type Actor%20Object%20Reference)))

(event EventTick
  (params (DeltaSeconds :type Float%20%28single-precision%29))
  ;[1 1 1] Audio follow player
  (bind _my_game_manager (CallFunction|GetMyGameManager))
  (Transformation|SetWorldTransform (Variables|Default|GetAudioCue) (Transformation|GetWorldTransform (Variables|/Script/Engine.Character|GetMesh (Variables|/Game/_ConvergencePoint/Blueprints/MyGameManager.MyGameManager_C|GetMyPlayer _my_game_manager))) false false))

(event EventInteract
  (params (PlayerInteracted :type Actor%20Object%20Reference))
  (bind _isoverlapping (CallFunction|IsOverlapping (Variables|Default|GetStatueCollision) PlayerInteracted))
  (if _isoverlapping
    (Utilities|FlowControl|FlipFlop
      (:A
        (bind _my_game_manager (CallFunction|GetMyGameManager))
        (Widget|RemovefromParent (Variables|/Game/_ConvergencePoint/Blueprints/MyGameManager.MyGameManager_C|GetInteractionWidget _my_game_manager))
        (Widget|SetVisibility (Variables|/Game/_ConvergencePoint/Blueprints/MyGameManager.MyGameManager_C|GetDialogWidget _my_game_manager) "Visible")
        (Audio|Components|Audio|Play (Variables|Default|GetAudioCue) 0.0)))))

(fn ConstructionScript)

(fn ShowHideWidget
  (params (Widget :type User%20Widget%20Object%20Reference) (Visibility :type ESlateVisibility%20Enum :default "Visible"))
  (Widget|SetVisibility Widget Visibility))