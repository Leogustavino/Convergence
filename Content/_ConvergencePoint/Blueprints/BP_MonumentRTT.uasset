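; BP_MonumentRTT is a render-to-texture stage that displays a selectable miniature object to a scene capture for rotatable viewing.
; SetMiniatureObject picks a mesh and uniform scale by ID from parallel lists, while PitchObject and TurnObject apply inverted pitch and yaw deltas to it.
; StartCapture resets the miniature's yaw relative to the player character and enables per-frame capture.
; StopCapture disables per-frame capture, so it runs only on demand.
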(event EventBeginPlay)

(event Collision|EventActorBeginOverlap
  (params (OtherActor :type Actor%20Object%20Reference)))

(event EventTick
  (params (DeltaSeconds :type Float%20%28single-precision%29)))

(fn ConstructionScript)

(fn SetMiniatureObject
  (params (ID :type Integer))
  (bind _miniatureobject (Variables|Default|GetMiniatureObject))
  (bind _listofobjectscale (Variables|Default|GetListOfObjectScale))
  (bind _output (Utilities|Array|Get(acopy) _listofobjectscale ID))
  (Components|StaticMesh|SetStaticMesh _miniatureobject (Utilities|Array|Get(acopy) (Variables|Default|GetListOfObjects) ID))
  (Transformation|SetWorldScale3D _miniatureobject (Math|Vector|MakeVector _output _output _output)))

(fn PitchObject
  (params (A :type Float%20%28single-precision%29))
  (Transformation|SetWorldRotation (Variables|Default|GetMiniatureObject) (Math|Rotator|CombineRotators (Transformation|GetWorldRotation (Variables|Default|GetMiniatureObject)) (Math|Rotator|MakeRotator 0.0 (* A -1.0) 0.0)) false false))

(fn TurnObject
  (params (A :type Float%20%28single-precision%29))
  (Transformation|SetWorldRotation (Variables|Default|GetMiniatureObject) (Math|Rotator|CombineRotators (Transformation|GetWorldRotation (Variables|Default|GetMiniatureObject)) (Math|Rotator|MakeRotator 0.0 0.0 (* A -1.0))) false false))

(fn StartCapture
  (CallFunction|ResetPosition)
  (Variables|/Script/Engine.SceneCaptureComponent|SetbCaptureEveryFrame (Variables|Default|GetSceneCaptureComponent2D) true))

(fn ResetPosition
  (bind _miniatureobject (Variables|Default|GetMiniatureObject))
  (bind _returnvalue (Transformation|GetWorldLocation _miniatureobject))
  (Transformation|SetWorldLocationAndRotation (Variables|Default|GetMiniatureObject) _returnvalue (Math|Rotator|MakeRotator 0.0 0.0 (+ (.Yaw (Math|Rotator|BreakRotator (Math|Rotator|FindLookatRotation _returnvalue (Transformation|GetActorLocation (Game|GetPlayerCharacter 0))))) 9e+01)) false false))

(fn StopCapture
  (Variables|/Script/Engine.SceneCaptureComponent|SetbCaptureEveryFrame (Variables|Default|GetSceneCaptureComponent2D) false))