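; BP_NewArea is a trigger volume that announces the player's arrival in a new area, with its box scaled by a variable at construction.
; Until the area is marked entered, a player overlap shows the HUD item counter and checks the dialogue BeatID.
; On beat two, it calls second-beat progression after a short delay and shows timed area and scan-objective messages, setting the entered flag only after they clear.
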(event OnComponentBeginOverlap(Box)
  (params (OverlappedComponent :type Primitive%20Component%20Object%20Reference) (OtherActor :type Actor%20Object%20Reference) (OtherComp :type Primitive%20Component%20Object%20Reference) (OtherBodyIndex :type Integer) (bFromSweep :type Boolean) (SweepResult :type Hit%20Result%20Structure%20%28by%20ref%29))
  (bind _my_game_manager (CallFunction|GetMyGameManager))
  (if (== (Variables|/Game/_ConvergencePoint/Blueprints/HighLevelBP/MyGameManager.MyGameManager_C|GetMyPlayer _my_game_manager) OtherActor)
    (if (not (Variables|Default|GethasEnteredNewArea?))
      (Widget|SetVisibility (Variables|/Game/_ConvergencePoint/Widgets/HUD.HUD_C|GetItemCounter (Variables|/Game/_ConvergencePoint/Blueprints/HighLevelBP/MyGameManager.MyGameManager_C|GetHUD _my_game_manager)) "Visible")
      (Utilities|FlowControl|Sequence
        (:then_0
          (CallFunction|TriggerBeat))
        (:then_1
          (CallFunction|NewAreaText (Variables|/Game/_ConvergencePoint/Blueprints/BP_Dialogue.BP_Dialogue_C|GetBeat_ID (Variables|/Game/_ConvergencePoint/Blueprints/HighLevelBP/MyGameManager.MyGameManager_C|GetDialogueBP _my_game_manager))))))))

(event Custom|TriggerBeat
  (bind _my_game_manager (CallFunction|GetMyGameManager))
  (if (== (Variables|/Game/_ConvergencePoint/Blueprints/BP_Dialogue.BP_Dialogue_C|GetBeat_ID (Variables|/Game/_ConvergencePoint/Blueprints/HighLevelBP/MyGameManager.MyGameManager_C|GetDialogueBP _my_game_manager)) 2)
    (Utilities|FlowControl|Delay 0.5)
    (Default|CallSecondBeatProgression)))

(event Custom|NewAreaText
  (params (Beat :type Integer))
  (if (== Beat 2)
    (Utilities|FlowControl|Delay 4.4)
    (bind _my_game_manager (CallFunction|GetMyGameManager))
    (Variables|/Game/_ConvergencePoint/Widgets/HUD.HUD_C|SetFeedbackText (Variables|/Game/_ConvergencePoint/Blueprints/HighLevelBP/MyGameManager.MyGameManager_C|GetHUD _my_game_manager) "Entered a new area")
    (Utilities|FlowControl|Delay 1.5)
    (Variables|/Game/_ConvergencePoint/Widgets/HUD.HUD_C|SetFeedbackText (Variables|/Game/_ConvergencePoint/Blueprints/HighLevelBP/MyGameManager.MyGameManager_C|GetHUD _my_game_manager) "3 items to scan")
    (Utilities|FlowControl|Delay 1.5)
    (Variables|/Game/_ConvergencePoint/Widgets/HUD.HUD_C|SetFeedbackText (Variables|/Game/_ConvergencePoint/Blueprints/HighLevelBP/MyGameManager.MyGameManager_C|GetHUD _my_game_manager) "")
    (Variables|Default|SethasEnteredNewArea? true)))

(event EventBeginPlay)

(event Collision|EventActorBeginOverlap
  (params (OtherActor :type Actor%20Object%20Reference)))

(event EventTick
  (params (DeltaSeconds :type Float%20%28single-precision%29)))

(fn ConstructionScript
  (Transformation|SetWorldScale3D (Variables|Default|GetBox) (Variables|Default|GetBoxCollisionScale)))

(fn UpdateCount)