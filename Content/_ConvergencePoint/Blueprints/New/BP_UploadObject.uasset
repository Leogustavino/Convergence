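; BP_UploadObject is an interactable upload pod that forwards player proximity and interaction to the game manager's UploadManager.
; CollisionBox overlaps show or hide the upload widget and Interact triggers the manager's interaction, all skipped in one specific player interaction state.
; AnimationBox overlaps toggle the pod animation regardless of state, and a separate PlayerInteraction function checks overlap before forwarding.
; The construction script scales CollisionBox from a Collision variable.
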(event OnComponentBeginOverlap(CollisionBox)
  (params (OverlappedComponent :type Primitive%20Component%20Object%20Reference) (OtherActor :type Actor%20Object%20Reference) (OtherComp :type Primitive%20Component%20Object%20Reference) (OtherBodyIndex :type Integer) (bFromSweep :type Boolean) (SweepResult :type Hit%20Result%20Structure%20%28by%20ref%29))
  (if (== OtherActor (Game|GetPlayerCharacter 0))
    (bind _my_game_manager (CallFunction|GetMyGameManager))
    (if (Utilities|Enum|NotEqual(Enum) (Variables|/Game/_ConvergencePoint/Blueprints/HighLevelBP/MyGameManager.MyGameManager_C|GetPlayer%20Interaction%20State _my_game_manager) "NewEnumerator7")
      (Default|DisplayWidget (Variables|/Game/_ConvergencePoint/Blueprints/HighLevelBP/MyGameManager.MyGameManager_C|GetUploadManager _my_game_manager)))))

(event OnComponentBeginOverlap(AnimationBox)
  (params (OverlappedComponent :type Primitive%20Component%20Object%20Reference) (OtherActor :type Actor%20Object%20Reference) (OtherComp :type Primitive%20Component%20Object%20Reference) (OtherBodyIndex :type Integer) (bFromSweep :type Boolean) (SweepResult :type Hit%20Result%20Structure%20%28by%20ref%29))
  (if (== OtherActor (Game|GetPlayerCharacter 0))
    (bind _my_game_manager (CallFunction|GetMyGameManager))
    (Default|UpdatePodAnimation (Variables|/Game/_ConvergencePoint/Blueprints/HighLevelBP/MyGameManager.MyGameManager_C|GetUploadManager _my_game_manager) true)))

(event OnComponentEndOverlap(CollisionBox)
  (params (OverlappedComponent :type Primitive%20Component%20Object%20Reference) (OtherActor :type Actor%20Object%20Reference) (OtherComp :type Primitive%20Component%20Object%20Reference) (OtherBodyIndex :type Integer))
  (if (== OtherActor (Game|GetPlayerCharacter 0))
    (bind _my_game_manager (CallFunction|GetMyGameManager))
    (if (Utilities|Enum|NotEqual(Enum) (Variables|/Game/_ConvergencePoint/Blueprints/HighLevelBP/MyGameManager.MyGameManager_C|GetPlayer%20Interaction%20State _my_game_manager) "NewEnumerator7")
      (Default|HideWidget (Variables|/Game/_ConvergencePoint/Blueprints/HighLevelBP/MyGameManager.MyGameManager_C|GetUploadManager _my_game_manager)))))

(event OnComponentEndOverlap(AnimationBox)
  (params (OverlappedComponent :type Primitive%20Component%20Object%20Reference) (OtherActor :type Actor%20Object%20Reference) (OtherComp :type Primitive%20Component%20Object%20Reference) (OtherBodyIndex :type Integer))
  (if (== OtherActor (Game|GetPlayerCharacter 0))
    (bind _my_game_manager (CallFunction|GetMyGameManager))
    (Default|UpdatePodAnimation (Variables|/Game/_ConvergencePoint/Blueprints/HighLevelBP/MyGameManager.MyGameManager_C|GetUploadManager _my_game_manager) false)))

(event EventBeginPlay)

(event Collision|EventActorBeginOverlap
  (params (OtherActor :type Actor%20Object%20Reference)))

(event EventTick
  (params (DeltaSeconds :type Float%20%28single-precision%29)))

(event EventInteract
  (params (PlayerInteracted :type Actor%20Object%20Reference))
  (bind _my_game_manager (CallFunction|GetMyGameManager))
  (if (Utilities|Enum|NotEqual(Enum) (Variables|/Game/_ConvergencePoint/Blueprints/HighLevelBP/MyGameManager.MyGameManager_C|GetPlayer%20Interaction%20State _my_game_manager) "NewEnumerator7")
    (Default|PlayerInteraction (Variables|/Game/_ConvergencePoint/Blueprints/HighLevelBP/MyGameManager.MyGameManager_C|GetUploadManager _my_game_manager))))

(fn ConstructionScript
  (Transformation|SetWorldScale3D (Variables|Default|GetCollisionBox) (Variables|Default|GetCollision)))

(fn PlayerInteraction
  (bind _my_game_manager (CallFunction|GetMyGameManager))
  (bind _isoverlapping (CallFunction|IsOverlapping (Variables|Default|GetCollisionBox) (Variables|/Game/_ConvergencePoint/Blueprints/HighLevelBP/MyGameManager.MyGameManager_C|GetMyPlayer _my_game_manager)))
  (if _isoverlapping
    (bind _my_game_manager_2 (CallFunction|GetMyGameManager))
    (Default|PlayerInteraction (Variables|/Game/_ConvergencePoint/Blueprints/HighLevelBP/MyGameManager.MyGameManager_C|GetUploadManager _my_game_manager_2))))