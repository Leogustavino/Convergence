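; Manager for scannable objects that tracks scan progress and triggers story beats.
; Loads descriptions from a data table into an array with scanned flags, counting unique monuments and collecting misc objects.
; A FlipFlop toggles inspection, switching object LODs, input, widget feedback and the GameManager's interaction state.
; Leaving collision at monument milestones fires delayed beat progressions; ending the pocket watch inspection after its beat 5 scan advances the story and destroys it.
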(event Custom|FithBeatA
  ;[1 1 1] Trigger - Fire Beat 5 A
  (Utilities|FlowControl|Delay 0.5)
  (Default|CallFifthBeatAProgression))

(event Custom|DestroyPocketWatch
  (bind _currentobject (Variables|Default|GetCurrentObject))
  ;[1 1 1] Trigger - Destroy pocket watch
  (if (Actor|ActorHasTag _currentobject "pocketwatch")
    (if (Variables|Default|GetPocketScanned?)
      (Default|CallFifthBeatCProgression)
      (Actor|DestroyActor _currentobject)
      ;[1 1 1] Update HUD item counter
      (bind _my_game_manager (CallFunction|GetMyGameManager))
      (Rendering|Components|TextRender|SetText (Variables|/Game/_ConvergencePoint/Widgets/MainWidgets/HUD.HUD_C|GetItemCounter (Variables|/Game/_ConvergencePoint/Blueprints/MyGameManager.MyGameManager_C|GetHUD _my_game_manager)) "100%"))))

(event Custom|DisplayWidget
  ;[1 1 1] Collide
  (CallFunction|DisplayObjectIntWidget)
  (bind _my_game_manager (CallFunction|GetMyGameManager))
  (Default|SetInsideCollisionBox (Variables|/Game/_ConvergencePoint/Blueprints/MyGameManager.MyGameManager_C|GetMyPlayer _my_game_manager) true)
  (if (Utilities|Enum|NotEqual(Enum) (Variables|/Game/_ConvergencePoint/Blueprints/MyGameManager.MyGameManager_C|GetPlayer%20Interaction%20State _my_game_manager) "NewEnumerator7")
    (Default|SetInteractionState _my_game_manager "NewEnumerator1" "NewEnumerator0")
    (else
      ;;[1 1 1] Hide "Scan E" whilst still in dialog
      (Widget|SetVisibility (Variables|Default|GetObjectInteractionWidget) "Collapsed"))))

(event Custom|HideWidget
  (bind _monumentscancount (Variables|Default|GetMonumentScanCount))
  ;[1 1 1] Exit collision
  (CallFunction|HideObjectIntWidget)
  (bind _my_game_manager (CallFunction|GetMyGameManager))
  (Default|SetInsideCollisionBox (Variables|/Game/_ConvergencePoint/Blueprints/MyGameManager.MyGameManager_C|GetMyPlayer _my_game_manager) false)
  (if (Utilities|Enum|NotEqual(Enum) (Variables|/Game/_ConvergencePoint/Blueprints/MyGameManager.MyGameManager_C|GetPlayer%20Interaction%20State _my_game_manager) "NewEnumerator7")
    (Default|SetInteractionState _my_game_manager "NewEnumerator0" "NewEnumerator0")
    (if (== _monumentscancount 1)
      (CallFunction|SecondBeatA)
      (elif (== _monumentscancount 6)
        (CallFunction|FithBeatA)))))

(event Custom|InteractWithObject
  (params (ID :type Integer) (InspectionObject :type Static%20Mesh%20Component%20Object%20Reference) (CurrentObject :type BP%20Interactable%20Object%20Parent%20Object%20Reference))
  (Utilities|FlowControl|FlipFlop
    (:A
      (Variables|Default|SetObjectID ID)
      (Variables|Default|SetCurrentObject CurrentObject)
      (Default|ChangeLODs CurrentObject true)
      (CallFunction|UpdateObjectIntWidget (Variables|Default|GetObjectID))
      (CallFunction|IncrementMonumentScanCount (Variables|Default|GetObjectID))
      (CallFunction|UpdateObject (Variables|Default|GetObjectID))
      (CallFunction|InsertMiscObjecttoArray (Variables|Default|GetObjectID))
      (Variables|Default|SetInspectionObject InspectionObject)
      (Input|EnableInput (Game|GetPlayerController 0))
      (bind _my_game_manager (CallFunction|GetMyGameManager))
      (Default|SetInteractionState _my_game_manager "NewEnumerator3" "NewEnumerator0")
      (Default|DisplayBorder (Variables|Default|GetObjectInteractionWidget) true))
    (:B
      (bind _my_game_manager_2 (CallFunction|GetMyGameManager))
      (if (Utilities|Enum|Equal(Enum) (Variables|/Game/_ConvergencePoint/Blueprints/MyGameManager.MyGameManager_C|GetPlayer%20Interaction%20State _my_game_manager_2) "NewEnumerator3")
        (Default|ChangeLODs CurrentObject false)
        (Default|FeedbackText (Variables|Default|GetObjectInteractionWidget) (Variables|/Game/_ConvergencePoint/Blueprints/New/BP_InteractableObjectParent.BP_InteractableObjectParent_C|GethasBeenScannedBefore? (Variables|Default|GetCurrentObject)))
        (Input|DisableInput (Game|GetPlayerController 0))
        (Default|SetInteractionState _my_game_manager_2 "NewEnumerator1" "NewEnumerator0")
        (Default|DisplayBorder (Variables|Default|GetObjectInteractionWidget) false)
        (Default|UpdateObjectScannedStatus (Variables|Default|GetCurrentObject) true)
        (CallFunction|DestroyPocketWatch)))))

(event Custom|SecondBeatA
  ;[1 1 1] Trigger  - Fire Beat 2 A
  (Utilities|FlowControl|Delay 0.5)
  (Default|CallSecondBeatAProgression))

(event EventBeginPlay
  (CallFunction|Init))

(event Input|ActionEvents|InputActionCloseWidget
  (params (Key :type Key%20Structure :default "None")))

(fn ConstructionScript)

(fn Init
  (bind _outrownames (DataTable|GetDataTableRowNames "/Game/_ConvergencePoint/Dialogue/ObjectDescriptionList.ObjectDescriptionList"))
  (for _array_element _outrownames
    (bind _returnvalue (Utilities|GetDataTableRow "/Game/_ConvergencePoint/Dialogue/ObjectDescriptionList.ObjectDescriptionList" _array_element)
      (:then
        (Utilities|Array|AddUnique (Variables|Default|GetObjectArray) (Utilities|Struct|MakeObjectStruct _returnvalue false))))))

(fn UpdateObject
  (params (ID :type Integer))
  (bind _objectarray (Variables|Default|GetObjectArray))
  (bind _output_get (LocalVariables|SetTempObject (Utilities|Struct|MakeObjectStruct (.ObjectDescriptionStruct (Utilities|Struct|BreakObjectStruct (Utilities|Array|Get(acopy) _objectarray ID))) true)))
  (Utilities|Array|SetArrayElem _objectarray ID _output_get)
  (if (== ID 6)
    (bind _my_game_manager (CallFunction|GetMyGameManager))
    (if (== (Variables|/Game/_ConvergencePoint/Blueprints/BP_Dialogue.BP_Dialogue_C|GetBeat_ID (Variables|/Game/_ConvergencePoint/Blueprints/MyGameManager.MyGameManager_C|GetDialogueBP _my_game_manager)) 5)
      (Variables|Default|SetPocketScanned? true))))

(fn DisplayObjectIntWidget
  (Utilities|IsValid (Variables|Default|GetObjectInteractionWidget)
    (:Is%20Valid
      (Widget|SetVisibility (Variables|Default|GetObjectInteractionWidget) "Visible"))
    (:Is%20Not%20Valid
      (bind _returnvalue (UserInterface|CreateWidget "/Game/_ConvergencePoint/Widgets/MainWidgets/ObjectInteractionWidget.ObjectInteractionWidget_C"))
      (bind _output_get (Variables|Default|SetObjectInteractionWidget _returnvalue))
      (UserInterface|Viewport|AddtoViewport _output_get 0))))

(fn HideObjectIntWidget
  (bind _objectinteractionwidget (Variables|Default|GetObjectInteractionWidget))
  (Utilities|IsValid _objectinteractionwidget
    (:Is%20Valid
      (Widget|SetVisibility _objectinteractionwidget "Hidden"))))

(fn UpdateObjectIntWidget
  (params (ID :type Integer))
  (Default|UpdateText (Variables|Default|GetObjectInteractionWidget) (.Description (Utilities|Struct|BreakObjectDescriptionStruct (.ObjectDescriptionStruct (Utilities|Struct|BreakObjectStruct (Utilities|Array|Get(acopy) (Variables|Default|GetObjectArray) ID)))))))

(fn OutputObjecttoInteract
  (return (Variables|Default|GetInspectionObject)))

(fn ResetObjectIntWidget
  (Default|ResetText (Variables|Default|GetObjectInteractionWidget)))

(fn IncrementMonumentScanCount
  (params (ID :type Integer))
  ;[1 1 1] Check for monument IDs
  (if (<= ID 5)
    ;[1 1 1] Only increment if not yet scanned
    (if (Math|Boolean|Equal(Boolean) (.HasBeenScanned? (Utilities|Struct|BreakObjectStruct (Utilities|Array|Get(acopy) (Variables|Default|GetObjectArray) ID))) false)
      (Math|Integer|IncrementInt (Variables|Default|GetMonumentScanCount)))))

(fn ReturnMonumentScanCount
  (return (Variables|Default|GetMonumentScanCount)))

(fn InsertMiscObjecttoArray
  (params (ID :type Integer))
  (bind _objectarray (Variables|Default|GetObjectArray))
  (bind _output (Utilities|Array|Get(acopy) _objectarray ID))
  (if (> ID 6)
    (if (.HasBeenScanned? (Utilities|Struct|BreakObjectStruct _output))
      (Utilities|Array|AddUnique (Variables|Default|GetMiscObjectArray) _output))))