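; Base interactable object that the player can highlight and interact with, using a configurable mesh shared by its world and inspection components.
; Detection overlap toggles a custom-depth stencil outline, while scan overlap shows or hides the ObjectManager widget.
; Interact, blocked in one game-manager interaction state, passes the object's ID and inspection mesh to ObjectManager after a scan-volume overlap check.
; ChangeLODs forces a different LOD while scanning; an older duplicate-mesh outline remains unexecuted.
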(event OnComponentBeginOverlap(ScanCollision)
  (params (OverlappedComponent :type Primitive%20Component%20Object%20Reference) (OtherActor :type Actor%20Object%20Reference) (OtherComp :type Primitive%20Component%20Object%20Reference) (OtherBodyIndex :type Integer) (bFromSweep :type Boolean) (SweepResult :type Hit%20Result%20Structure%20%28by%20ref%29))
  (if (== OtherActor (Game|GetPlayerCharacter 0))
    (bind _my_game_manager (CallFunction|GetMyGameManager))
    (Default|DisplayWidget (Variables|/Game/_ConvergencePoint/Blueprints/HighLevelBP/MyGameManager.MyGameManager_C|GetObjectManager _my_game_manager))))

(event OnComponentEndOverlap(ScanCollision)
  (params (OverlappedComponent :type Primitive%20Component%20Object%20Reference) (OtherActor :type Actor%20Object%20Reference) (OtherComp :type Primitive%20Component%20Object%20Reference) (OtherBodyIndex :type Integer))
  (if (== OtherActor (Game|GetPlayerCharacter 0))
    (bind _my_game_manager (CallFunction|GetMyGameManager))
    (Default|HideWidget (Variables|/Game/_ConvergencePoint/Blueprints/HighLevelBP/MyGameManager.MyGameManager_C|GetObjectManager _my_game_manager))))

(event OnComponentBeginOverlap(DetectionCollision)
  (params (OverlappedComponent :type Primitive%20Component%20Object%20Reference) (OtherActor :type Actor%20Object%20Reference) (OtherComp :type Primitive%20Component%20Object%20Reference) (OtherBodyIndex :type Integer) (bFromSweep :type Boolean) (SweepResult :type Hit%20Result%20Structure%20%28by%20ref%29))
  (if (== OtherActor (Game|GetPlayerCharacter 0))
    (CallFunction|GetMyGameManager)
    (CallFunction|DrawOutline (Variables|Default|GetObject))))

(event OnComponentEndOverlap(DetectionCollision)
  (params (OverlappedComponent :type Primitive%20Component%20Object%20Reference) (OtherActor :type Actor%20Object%20Reference) (OtherComp :type Primitive%20Component%20Object%20Reference) (OtherBodyIndex :type Integer))
  (if (== OtherActor (Game|GetPlayerCharacter 0))
    (CallFunction|GetMyGameManager)
    (CallFunction|EraseOutline)))

(event EventInteract
  (params (PlayerInteracted :type Actor%20Object%20Reference))
  (bind _my_game_manager (CallFunction|GetMyGameManager))
  (if (Utilities|Enum|NotEqual(Enum) (Variables|/Game/_ConvergencePoint/Blueprints/HighLevelBP/MyGameManager.MyGameManager_C|GetPlayer%20Interaction%20State _my_game_manager) "NewEnumerator7")
    (CallFunction|PlayerInteraction PlayerInteracted false)))

(fn ConstructionScript
  (bind _mesh (Variables|Default|GetMesh))
  (bind _inspection_mesh_scale (Variables|Default|GetInspection%20Mesh%20Scale))
  (Components|StaticMesh|SetStaticMesh (Variables|Default|GetObject) _mesh)
  (Components|StaticMesh|SetStaticMesh (Variables|Default|GetInspectionMesh) _mesh)
  (Transformation|SetWorldScale3D (Variables|Default|GetScanCollision) (Variables|Default|GetScanCollisionScale))
  (Transformation|SetWorldScale3D (Variables|Default|GetInspectionMesh) (Math|Vector|MakeVector _inspection_mesh_scale _inspection_mesh_scale _inspection_mesh_scale))
  (Transformation|SetWorldScale3D (Variables|Default|GetDetectionCollision) (Variables|Default|GetDetectionCollisionScale)))

(fn PlayerInteraction
  (params (PlayerInteracted :type Object%20Object%20Reference) (isScanning? :type Boolean))
  (bind _isoverlapping (CallFunction|IsOverlapping (Variables|Default|GetScanCollision) PlayerInteracted))
  (if _isoverlapping
    (bind _my_game_manager (CallFunction|GetMyGameManager))
    (Default|InteractwithObject (Variables|/Game/_ConvergencePoint/Blueprints/HighLevelBP/MyGameManager.MyGameManager_C|GetObjectManager _my_game_manager) (Variables|Default|GetObjectID) (Variables|Default|GetInspectionMesh) self)))

(fn DrawOutline
  (params (Outline%20Mesh :type Static%20Mesh%20Component%20Object%20Reference))
  (bind _object (Variables|Default|GetObject))
  (Rendering|SetRenderCustomDepth _object true)
  (Rendering|SetCustomDepthStencilValue _object 2))

(fn EraseOutline
  (bind _object (Variables|Default|GetObject))
  (Rendering|SetRenderCustomDepth _object false)
  (Rendering|SetCustomDepthStencilValue _object 0))

(fn ChangeLODs
  (params (Scanning? :type Boolean))
  (if Scanning?
    (Rendering|LOD|SetForcedLodModel (Variables|Default|GetObject) 4)
    (else
      (Rendering|LOD|SetForcedLodModel (Variables|Default|GetObject) 0))))