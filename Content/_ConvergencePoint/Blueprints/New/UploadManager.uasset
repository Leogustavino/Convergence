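; Manages the scan upload step, showing and hiding the upload widget and updating the game manager's interaction state.
; On interaction, it tallies scanned statue and sphinx items by their index in the ObjectManager array.
; The dialogue BeatID selects the required set, with the second upload also needing the pocket watch.
; The widget shows the count or success text, and a successful upload fires delayed third or sixth beat progression.
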(event Custom|DisplayWidget
  (CallFunction|DisplayUploadWidget)
  (bind _my_game_manager (CallFunction|GetMyGameManager))
  (if (Utilities|Enum|NotEqual(Enum) (Variables|/Game/_ConvergencePoint/Blueprints/HighLevelBP/MyGameManager.MyGameManager_C|GetPlayer%20Interaction%20State _my_game_manager) "NewEnumerator7")
    (Default|SetInteractionState _my_game_manager "NewEnumerator1" "NewEnumerator1")))

(event Custom|HideWidget
  (CallFunction|HideUploadWidget)
  (bind _my_game_manager (CallFunction|GetMyGameManager))
  (if (Utilities|Enum|NotEqual(Enum) (Variables|/Game/_ConvergencePoint/Blueprints/HighLevelBP/MyGameManager.MyGameManager_C|GetPlayer%20Interaction%20State _my_game_manager) "NewEnumerator7")
    (Default|SetInteractionState _my_game_manager "NewEnumerator0" "NewEnumerator1")))

(event Custom|PlayerInteraction
  ;[1 1 1] Retrieve Count
  (CallFunction|CheckCounter)
  ;[1 1 1] Update counter depending on beat
  (bind _my_game_manager (CallFunction|GetMyGameManager))
  (CallFunction|CheckSuccessfulUpload (Variables|/Game/_ConvergencePoint/Blueprints/BP_Dialogue.BP_Dialogue_C|GetBeat_ID (Variables|/Game/_ConvergencePoint/Blueprints/HighLevelBP/MyGameManager.MyGameManager_C|GetDialogueBP _my_game_manager)))
  (CallFunction|UpdateTextCounter (Variables|/Game/_ConvergencePoint/Blueprints/BP_Dialogue.BP_Dialogue_C|GetBeat_ID (Variables|/Game/_ConvergencePoint/Blueprints/HighLevelBP/MyGameManager.MyGameManager_C|GetDialogueBP _my_game_manager)))
  (CallFunction|ResetCounter)
  (Default|SetInteractionState _my_game_manager "NewEnumerator4" "NewEnumerator1"))

(event Custom|Fire3rdBeat
  (Utilities|FlowControl|Delay 4.0)
  (Default|Call3rdBeatProgression))

(event Custom|Fire6thBeat
  (Utilities|FlowControl|Delay 4.0)
  (Default|Call6thBeatProgression))

(event Custom|UpdatePodAnimation
  (params (InsideCollision? :type Boolean))
  (Variables|Default|SetInsideCollision? InsideCollision?))

(event Custom|PlayerInput
  (CallFunction|DisplayUploadWidget)
  (CallFunction|CheckCounter)
  (bind _my_game_manager (CallFunction|GetMyGameManager))
  (CallFunction|UpdateTextCounter (Variables|/Game/_ConvergencePoint/Blueprints/BP_Dialogue.BP_Dialogue_C|GetBeat_ID (Variables|/Game/_ConvergencePoint/Blueprints/HighLevelBP/MyGameManager.MyGameManager_C|GetDialogueBP _my_game_manager)))
  (CallFunction|CheckSuccessfulUpload (Variables|/Game/_ConvergencePoint/Blueprints/BP_Dialogue.BP_Dialogue_C|GetBeat_ID (Variables|/Game/_ConvergencePoint/Blueprints/HighLevelBP/MyGameManager.MyGameManager_C|GetDialogueBP _my_game_manager)))
  (Utilities|FlowControl|Delay 2.0)
  (CallFunction|HideUploadWidget))

(fn ConstructionScript)

(fn DisplayUploadWidget
  (Utilities|IsValid (Variables|Default|GetUploadWidget)
    (:Is%20Valid
      (Widget|SetVisibility (Variables|Default|GetUploadWidget) "Visible"))
    (:Is%20Not%20Valid
      (bind _returnvalue (UserInterface|CreateWidget "/Game/_ConvergencePoint/Widgets/UploadWidget.UploadWidget_C"))
      (bind _output_get (Variables|Default|SetUploadWidget _returnvalue))
      (UserInterface|Viewport|AddtoViewport _output_get 0))))

(fn HideUploadWidget
  (Utilities|IsValid (Variables|Default|GetUploadWidget)
    (:Is%20Valid
      (Widget|RemovefromParent (Variables|Default|GetUploadWidget))
      (Variables|Default|SetUploadWidget 0))))

(fn UpdateTextCounter
  (params (beat_ID :type Integer))
  (bind _returnvalue (<= beat_ID 6))
  (bind _returnvalue_2 (<= beat_ID 3))
  (if (Variables|Default|GetSuccessfulUpload)
    (if _returnvalue_2
      (Default|SuccessfulUploadText (Variables|Default|GetUploadWidget) 50)
      (elif _returnvalue
        (Default|SuccessfulUploadText (Variables|Default|GetUploadWidget) 100)))
    (elif _returnvalue_2
      (LocalVariables|SetCount (Variables|Default|GetStatueCount))
      (Default|CreateText (Variables|Default|GetUploadWidget) (LocalVariables|GetCount) :!label _label)
      (elif _returnvalue
        (LocalVariables|SetCount (Variables|Default|GetSphinxCount))
        (goto _label)))))

(fn ResetTextCounter
  (Variables|/Game/_ConvergencePoint/Widgets/UploadWidget.UploadWidget_C|SetFinalText (Variables|Default|GetUploadWidget) ""))

(fn CheckCounter
  (bind _my_game_manager (CallFunction|GetMyGameManager))
  (bind (_array_element _array_index) (Utilities|Array|ForEachLoopwithBreak (Variables|/Game/_ConvergencePoint/Blueprints/New/ObjectManager.ObjectManager_C|GetObjectArray (Variables|/Game/_ConvergencePoint/Blueprints/HighLevelBP/MyGameManager.MyGameManager_C|GetObjectManager _my_game_manager)) :!label _label)
    (:LoopBody
      ;[1 1 1] First 3 items - Statue
      (if (< _array_index 3)
        (if (.HasBeenScanned? (Utilities|Struct|BreakObjectStruct _array_element))
          (Variables|Default|SetStatueCount (+ (Variables|Default|GetStatueCount) 1)))
        (else
          ;[1 1 1] Items 4-6 - Sphinx
          (if (< _array_index 6)
            (if (.HasBeenScanned? (Utilities|Struct|BreakObjectStruct _array_element))
              (Math|Integer|IncrementInt (Variables|Default|GetSphinxCount)))
            (else
              (goto _label Break))))))))

(fn ResetCounter
  (Variables|Default|SetStatueCount 0)
  (Variables|Default|SetSphinxCount 0))

(fn CheckSuccessfulUpload
  (params (Beat_ID :type Integer))
  (if (<= Beat_ID 3)
    (if (== (Variables|Default|GetStatueCount) 3)
      (LocalVariables|SetTemp true)
      (Default|UpdateUploadText (Variables|Default|GetUploadWidget))
      (CallFunction|Fire3rdBeat)
      (Variables|Default|SetSuccessfulUpload true)
      (else
        (LocalVariables|SetTemp false)
        (Variables|Default|SetSuccessfulUpload false)))
    (elif (== Beat_ID 6)
      (bind _my_game_manager (CallFunction|GetMyGameManager))
      (if (and (== (Variables|Default|GetSphinxCount) 3) (Math|Boolean|Equal(Boolean) (Variables|/Game/_ConvergencePoint/Blueprints/New/ObjectManager.ObjectManager_C|GetPocketScanned? (Variables|/Game/_ConvergencePoint/Blueprints/HighLevelBP/MyGameManager.MyGameManager_C|GetObjectManager _my_game_manager)) true))
        (LocalVariables|SetTemp true)
        (Default|UpdateUploadText (Variables|Default|GetUploadWidget))
        (CallFunction|Fire6thBeat)
        (Variables|Default|SetSuccessfulUpload true)
        (else
          (LocalVariables|SetTemp false :!label _label)
          (Variables|Default|SetSuccessfulUpload false)))
      (else
        (goto _label)))))

(fn ResetSuccessfulUpload
  (params (Condition :type Boolean))
  (if Condition
    (Variables|Default|SetSuccessfulUpload false)))