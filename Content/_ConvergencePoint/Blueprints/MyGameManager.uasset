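; Game manager Blueprint that tracks the game state (Running, Won, Abandon) and owns the main UI widgets.
; On BeginPlay it creates the abandon, interaction, dialog, upload and HUD widgets, then requests Running.
; SetState acts only on a change, hiding all UI before toggling the HUD or abandon screen and mouse; Won only prints.
; Monument helpers are unfinished: an empty setter, a fixed-value getter and a debug-print scan check.
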(event EventBeginPlay
  (CallFunction|Init self))

(event Collision|EventActorBeginOverlap
  (params (OtherActor :type Actor%20Object%20Reference)))

(event EventTick
  (params (DeltaSeconds :type Float%20%28single-precision%29)))

(fn ConstructionScript)

(fn Init
  (CallFunction|CreateUI)
  (CallFunction|SetState "NewEnumerator0"))

(fn SetState
  (params (New%20State :type MyGameStates%20Enum :default "NewEnumerator0"))
  (if (Utilities|Enum|NotEqual(Enum) New%20State (Variables|Default|GetCurrent%20Game%20State))
    (CallFunction|HideUI)
    (bind _output_get (Variables|Default|SetCurrent%20Game%20State New%20State))
    (switch Utilities|FlowControl|Switch|SwitchonMyGameStates _output_get
      (:NewEnumerator0
        (CallFunction|ShowMouse false)
        (Widget|SetVisibility (Variables|Widgets|GetHUD) "Visible"))
      (:NewEnumerator1
        (Development|PrintString "You won the game"))
      (:NewEnumerator3
        (Widget|SetVisibility (Variables|Widgets|GetWidget_Abandon) "Visible")
        (CallFunction|ShowMouse true)
        (Development|PrintString "lost")))))

(fn GetState
  (return (Variables|Default|GetCurrent%20Game%20State)))

(fn CreateUI
  (bind _returnvalue (UserInterface|CreateWidget "/Game/_ConvergencePoint/Widgets/Widget_Abandon.Widget_Abandon_C"))
  (bind _output_get (Variables|Widgets|SetWidget_Abandon _returnvalue))
  (UserInterface|Viewport|AddtoViewport _output_get 0)
  (bind _widget (CallFunction|InitWidget "/Game/_ConvergencePoint/Widgets/InteractionWidget.InteractionWidget_C"))
  (Variables|Widgets|SetInteractionWidget _widget)
  (bind _widget_2 (CallFunction|InitWidget "/Game/_ConvergencePoint/Widgets/DialogWidget.DialogWidget_C"))
  (Variables|Widgets|SetDialogWidget _widget_2)
  (bind _widget_3 (CallFunction|InitWidget "/Game/_ConvergencePoint/Widgets/UploadWidget.UploadWidget_C"))
  (Variables|Widgets|SetUploadWidget _widget_3)
  (bind _widget_4 (CallFunction|InitWidget "/Game/_ConvergencePoint/Widgets/HUD.HUD_C"))
  (Variables|Widgets|SetHUD _widget_4))

(fn SetMonument)

(fn GetMonument
  (bind _output_get (Variables|Monuments|SetObjectSelection (Variables|/Game/_ConvergencePoint/Blueprints/BP_InteractParent.BP_InteractParent_C|GetMonument (Variables|Monuments|GetInteractableObject))))
  (return _output_get))

(fn MonumentScanned?
  (bind _values (Utilities|Map|Values (Variables|Default|GetMonumentScanned)))
  (for _array_element _values
    (if _array_element
      (Development|PrintString "Hello"))))