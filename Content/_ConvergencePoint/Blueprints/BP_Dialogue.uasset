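; Dialogue director Blueprint that drives the game's scripted story beats, from the opening dialogue to the credits.
; Each beat calls its play dispatcher, shows timed subtitles while changing interaction state, then binds the next beat to events from area, object and upload managers or dialogue triggers.
; Beats also advance a beat counter and fire side effects like camera shakes, flashlight unlock and a logbook update.
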(event Custom|2ndBeatA
  (Default|CallPlaySecondBeatA)
  (EventDispatchers|UnbindEventfromSecondBeatAProgression (Variables|/Game/_ConvergencePoint/Blueprints/MyGameManager.MyGameManager_C|GetObjectManager (stale Custom|2ndbeat _my_game_manager)) (delegate Custom|2ndBeatA))
  (CallFunction|DisplaySubtitleWidget 5.3)
  (CallFunction|IncrementBeatCount)
  (bind _my_game_manager (CallFunction|GetMyGameManager))
  (EventDispatchers|BindEventto3rdBeatProgression (Variables|/Game/_ConvergencePoint/Blueprints/MyGameManager.MyGameManager_C|GetUploadManager _my_game_manager) (delegate Custom|3rdBeat)))

(event Custom|4thBeatA
  (Default|CallPlayFourthBeatA)
  (CallFunction|DisplaySubtitleWidget 6.7)
  (bind _my_game_manager (CallFunction|GetMyGameManager))
  (EventDispatchers|BindEventtoFourthBBeatProgression (Variables|/Game/_ConvergencePoint/Blueprints/MyGameManager.MyGameManager_C|GetNewArea _my_game_manager) (delegate Custom|4thBeatB))
  ;[1 1 1] FX camera shake/flashlight enabled
  (CallFunction|CameraShake 3.0)
  ;;[1 1 1] Flashlight enabled
  (Utilities|FlowControl|Delay 6.0)
  (Default|EnableFlashlight (Variables|/Game/_ConvergencePoint/Blueprints/MyGameManager.MyGameManager_C|GetMyPlayer _my_game_manager))
  (Default|EnableFlashlight (Variables|/Game/_ConvergencePoint/Blueprints/MyGameManager.MyGameManager_C|GetHUD _my_game_manager))
  (Default|EnabledFlashText (Variables|/Game/_ConvergencePoint/Blueprints/MyGameManager.MyGameManager_C|GetHUD _my_game_manager)))

(event Custom|6thbeat
  (Default|CallPlaySixthBeat)
  (EventDispatchers|UnbindEventfrom6thBeatProgression (Variables|/Game/_ConvergencePoint/Blueprints/MyGameManager.MyGameManager_C|GetUploadManager (stale Custom|5thBeatC _my_game_manager)) (delegate Custom|6thbeat))
  (CallFunction|DisplaySubtitleWidget 32.400002)
  (CallFunction|IncrementBeatCount)
  (Utilities|FlowControl|Delay 33.0)
  (bind _returnvalue (UserInterface|CreateWidget "/Game/_ConvergencePoint/Widgets/MainWidgets/CreditsWidget.CreditsWidget_C"))
  (bind _output_get (Variables|Default|SetcreditWidget _returnvalue))
  (UserInterface|Viewport|AddtoViewport _output_get 0)
  (Default|StartAnimation _output_get))

(event Custom|cameraShake
  (params (Delay :type Float%20%28single-precision%29))
  (Utilities|FlowControl|Delay Delay)
  (Camera|PlayWorldCameraShake "/Game/_ConvergencePoint/Blueprints/MyShake.MyShake_C" (Transformation|GetActorLocation (Game|GetPlayerCharacter 0)) 0.0 5e+02))

(event Custom|StartDialog
  ;[1 1 1] Act 1
  (CallFunction|DisplaySubtitleWidget 29.0)
  (bind _my_game_manager (CallFunction|GetMyGameManager))
  (CallFunction|IncrementBeatCount)
  (EventDispatchers|BindEventtoSecondBeatProgression (Variables|/Game/_ConvergencePoint/Blueprints/MyGameManager.MyGameManager_C|GetNewArea _my_game_manager) (delegate Custom|2ndbeat))
  ;[1 1 1] FX - Camera shake
  (CallFunction|CameraShake 5.7))

(event Custom|4thBeatB
  (Default|CallPlayFourthBeatB)
  (CallFunction|DisplaySubtitleWidget 3.4)
  (CallFunction|IncrementBeatCount)
  (bind _my_game_manager (CallFunction|GetMyGameManager))
  (EventDispatchers|BindEventtoFifthBeatAProgression (Variables|/Game/_ConvergencePoint/Blueprints/MyGameManager.MyGameManager_C|GetObjectManager _my_game_manager) (delegate Custom|5thBeatA)))

(event Custom|5thBeatA
  (Default|CallPlayFifthBeatA)
  (EventDispatchers|UnbindEventfromFifthBeatAProgression (Variables|/Game/_ConvergencePoint/Blueprints/MyGameManager.MyGameManager_C|GetObjectManager (stale Custom|4thBeatB _my_game_manager)) (delegate Custom|5thBeatA))
  (CallFunction|DisplaySubtitleWidget 7.3)
  (bind _returnvalue (Actor|GetActorOfClass "/Game/_ConvergencePoint/Blueprints/Triggers/BP_DialogueTrigger_OutsideTrain.BP_DialogueTrigger_OutsideTrain_C"))
  (EventDispatchers|BindEventto5thBeatBProgression _returnvalue (delegate Custom|5thBeatB))
  ;[1 1 1] Update logbook
  (bind _my_game_manager (CallFunction|GetMyGameManager))
  (bind _asmain_logbook_widget (Utilities|Casting|CastToMainLogbookWidget (Variables|/Game/_ConvergencePoint/Blueprints/MyGameManager.MyGameManager_C|GetLogbook _my_game_manager)))
  (Default|UpdatePocketWatch _asmain_logbook_widget))

(event Custom|2ndbeat
  (Default|CallPlaySecondBeat)
  (EventDispatchers|UnbindEventfromSecondBeatProgression (Variables|/Game/_ConvergencePoint/Blueprints/MyGameManager.MyGameManager_C|GetNewArea (stale Custom|StartDialog _my_game_manager)) (delegate Custom|2ndbeat))
  (CallFunction|DisplaySubtitleWidget 6.0)
  (bind _my_game_manager (CallFunction|GetMyGameManager))
  (EventDispatchers|BindEventtoSecondBeatAProgression (Variables|/Game/_ConvergencePoint/Blueprints/MyGameManager.MyGameManager_C|GetObjectManager _my_game_manager) (delegate Custom|2ndBeatA)))

(event Custom|5thBeatB
  (Default|CallPlayFifthBeatB)
  (CallFunction|DisplaySubtitleWidget 3.8)
  (EventDispatchers|BindEventtoFifthBeatCProgression (Variables|/Game/_ConvergencePoint/Blueprints/MyGameManager.MyGameManager_C|GetObjectManager (stale Custom|4thBeatB _my_game_manager)) (delegate Custom|5thBeatC)))

(event Custom|3rdBeat
  (Default|CallPlayThirdBeat)
  (bind _my_game_manager (CallFunction|GetMyGameManager))
  (EventDispatchers|UnbindEventfrom3rdBeatProgression (Variables|/Game/_ConvergencePoint/Blueprints/MyGameManager.MyGameManager_C|GetUploadManager _my_game_manager) (delegate Custom|3rdBeat))
  (CallFunction|DisplaySubtitleWidget 16.700001)
  (CallFunction|IncrementBeatCount)
  (bind _returnvalue (Actor|GetActorOfClass "/Game/_ConvergencePoint/Blueprints/Triggers/BP_DialogueTrigger.BP_DialogueTrigger_C"))
  (EventDispatchers|BindEventto4thBeatABeatProgression _returnvalue (delegate Custom|4thBeatA)))

(event Custom|5thBeatC
  (Default|CallPlayFifthBeatC)
  (CallFunction|DisplaySubtitleWidget 4.2)
  (CallFunction|IncrementBeatCount)
  (bind _my_game_manager (CallFunction|GetMyGameManager))
  (EventDispatchers|BindEventto6thBeatProgression (Variables|/Game/_ConvergencePoint/Blueprints/MyGameManager.MyGameManager_C|GetUploadManager _my_game_manager) (delegate Custom|6thbeat)))

(event Custom|DisplaySubtitleWidget
  (params (Duration :type Float%20%28single-precision%29))
  ;[1 1 1 1 66] DisplayWidget and pause interaction
  (Variables|Default|SetisDialoguePlaying? true)
  (bind _my_game_manager (CallFunction|GetMyGameManager))
  (Widget|SetVisibility (Variables|/Game/_ConvergencePoint/Blueprints/SubtitlesManager.SubtitlesManager_C|GetSubtitlesWidgetRef (Variables|/Game/_ConvergencePoint/Blueprints/MyGameManager.MyGameManager_C|GetSubtitleManager _my_game_manager)) "Visible")
  (Default|SetInteractionState _my_game_manager "NewEnumerator7" "NewEnumerator0")
  (Utilities|FlowControl|Delay Duration)
  (Default|ClearSubtitles (Variables|/Game/_ConvergencePoint/Blueprints/MyGameManager.MyGameManager_C|GetSubtitleManager _my_game_manager))
  (Default|SetInteractionState _my_game_manager "NewEnumerator0" "NewEnumerator0")
  (Variables|Default|SetisDialoguePlaying? false))

(fn ConstructionScript)

(fn IncrementBeatCount
  (Math|Integer|IncrementInt (Variables|Default|GetBeat_ID)))

(fn UpdateBeatCount
  (params (Successful%20Upload :type Boolean))
  (if Successful%20Upload
    (CallFunction|IncrementBeatCount)))