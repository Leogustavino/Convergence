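; Game manager Blueprint that owns the UI widgets, game state, player interaction state and monument scan and upload progress.
; On BeginPlay it creates the HUD, abandon, interaction, dialog, upload, logbook and narrative widgets, then enters Running.
; Two switch-based state setters hide all UI, then show matching widgets and adjust cursor or player movement.
; Other functions track counts and trigger narrative progression; the scanned-monument check and win state only print debug text.
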(event EventBeginPlay
  (CallFunction|Init self))

(event Collision|EventActorBeginOverlap
  (params (OtherActor :type Actor%20Object%20Reference)))

(event EventTick
  (params (DeltaSeconds :type Float%20%28single-precision%29)))

(fn ConstructionScript)

(fn Init
  (CallFunction|CreateUI)
  (CallFunction|SetState "NewEnumerator0"))

(fn SetState
  (params (New%20State :type MyGameStates%20Enum :default "NewEnumerator0"))
  (if (Utilities|Enum|NotEqual(Enum) New%20State (Variables|Default|GetCurrent%20Game%20State))
    (CallFunction|HideUI)
    (bind _output_get (Variables|Default|SetCurrent%20Game%20State New%20State))
    (switch Utilities|FlowControl|Switch|SwitchonMyGameStates _output_get
      (:NewEnumerator0
        (CallFunction|ShowMouse false)
        (Widget|SetVisibility (Variables|Widgets|GetHUD) "Visible"))
      (:NewEnumerator1
        (Development|PrintString "You won the game"))
      (:NewEnumerator3
        (Widget|SetVisibility (Variables|Widgets|GetWidget_Abandon) "Visible")
        (CallFunction|ShowMouse true)))))

(fn GetState
  (return (Variables|Default|GetCurrent%20Game%20State)))

(fn CreateUI
  (bind _returnvalue (UserInterface|CreateWidget "/Game/_ConvergencePoint/Widgets/Widget_Abandon.Widget_Abandon_C"))
  (bind _output_get (Variables|Widgets|SetWidget_Abandon _returnvalue))
  (UserInterface|Viewport|AddtoViewport _output_get 0)
  (bind _widget (CallFunction|InitWidget "/Game/_ConvergencePoint/Widgets/InteractionWidget.InteractionWidget_C"))
  (Variables|Widgets|SetInteractionWidget _widget)
  (bind _widget_2 (CallFunction|InitWidget "/Game/_ConvergencePoint/Widgets/DialogWidget.DialogWidget_C"))
  (Variables|Widgets|SetDialogWidget _widget_2)
  (bind _widget_3 (CallFunction|InitWidget "/Game/_ConvergencePoint/Widgets/UploadWidget.UploadWidget_C"))
  (Variables|Widgets|SetUploadWidget _widget_3)
  (bind _widget_4 (CallFunction|InitWidget "/Game/_ConvergencePoint/Widgets/HUD.HUD_C"))
  (Variables|Widgets|SetHUD _widget_4)
  (bind _widget_5 (CallFunction|InitWidget "/Game/_ConvergencePoint/Widgets/LogbookWidget.LogbookWidget_C"))
  (Variables|Widgets|SetLogbook _widget_5)
  (bind _widget_6 (CallFunction|InitWidget "/Game/_ConvergencePoint/Widgets/NarrativeBeatWidget.NarrativeBeatWidget_C"))
  (Variables|Widgets|SetNarrativeBeatWidget _widget_6))

(fn SetMonument
  (bind _output_get (Variables|Monuments|SetObjectSelection (Variables|/Game/_ConvergencePoint/Blueprints/BP_InteractParent.BP_InteractParent_C|GetMonument (Variables|Monuments|GetInteractableObject))))
  (return _output_get))

(fn GetMonument
  (return (Variables|Monuments|GetObjectSelection)))

(fn MonumentScanned?
  (bind _values (Utilities|Map|Values (Variables|Monuments|GetMonumentScanned)))
  (for _array_element _values
    (if _array_element
      (Development|PrintString "Hello"))))

(fn SetInteractionState
  (params (Input :type PlayerInputInteractionStates%20Enum :default "NewEnumerator0"))
  (bind _myplayer (Variables|Default|GetMyPlayer))
  (bind _hud (Variables|Widgets|GetHUD))
  (bind _myplayer_2 (Variables|Default|GetMyPlayer))
  (if (Utilities|Enum|NotEqual(Enum) Input (Variables|Default|GetPlayer%20Interaction%20State))
    (CallFunction|HideUI)
    (bind _output_get (Variables|Default|SetPlayer%20Interaction%20State Input))
    (switch Utilities|FlowControl|Switch|SwitchonPlayerInputInteractionStates _output_get
      (:NewEnumerator0
        ;[1 1 1] Neutral
        (Widget|SetVisibility _hud "Visible")
        (Default|EnableMovement _myplayer)
        (CallFunction|ShowMouse false)
        (Variables|/Game/FirstPersonBP/Blueprints/FirstPersonCharacter.FirstPersonCharacter_C|SetHasMenuOpen? _myplayer false))
      (:NewEnumerator1
        ;[1 1 1] Logbook open
        (Widget|SetVisibility (Variables|Widgets|GetLogbook) "Visible")
        (Default|DisableMovement _myplayer_2)
        (CallFunction|ShowMouse true)
        (Variables|/Game/FirstPersonBP/Blueprints/FirstPersonCharacter.FirstPersonCharacter_C|SetHasMenuOpen? _myplayer_2 true))
      (:NewEnumerator2
        (Widget|SetVisibility (Variables|Widgets|GetInteractionWidget) "Visible")
        (Widget|SetVisibility _hud "Visible"))
      (:NewEnumerator3
        (Widget|SetVisibility (Variables|Widgets|GetDialogWidget) "Visible")))))

(fn GetInteractionState
  (return (Variables|Default|GetPlayer%20Interaction%20State)))

(fn IncreaseMonumentCount
  (params (MonumentSelection :type InteractableObjects_Enum%20Enum :default "NewEnumerator8"))
  (if (not (.Value (Utilities|Map|Find (Variables|Monuments|GetMonumentScanned) MonumentSelection)))
    (Math|Integer|IncrementInt (Variables|GameProgression|GetMonumentCount))))

(fn IncreaseUploadCount
  (Math|Integer|IncrementInt (Variables|GameProgression|GetUploadCount)))

(fn ProgressStory
  (Default|CallProgressNarrativeBeat))