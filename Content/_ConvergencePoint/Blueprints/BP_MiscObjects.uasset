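; BP_MiscObjects is an interactable, inspectable world object that can be scanned and recorded in the player's logbook.
; Player overlap toggles an outline on the inspection mesh, and the construction script applies one mesh to both interactable and inspection components and caches the child-actor scanner.
; Interact runs the player interaction, then, if the player is inspecting, starts the scan and adds the object's struct uniquely to the player's inventory.
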(event EventBeginPlay
  (|CallParentFunction))

(event Collision|EventActorBeginOverlap
  (params (OtherActor :type Actor%20Object%20Reference))
  (if (== OtherActor (Game|GetPlayerCharacter 0))
    (CallFunction|BeginOverlap OtherActor)
    (CallFunction|DrawOutline (Variables|Default|GetInspectionMesh))))

(event EventInteract
  (params (PlayerInteracted :type Actor%20Object%20Reference))
  (CallFunction|PlayerInteraction PlayerInteracted "NewEnumerator8")
  (bind _my_game_manager (CallFunction|GetMyGameManager))
  (if (Variables|/Game/FirstPersonBP/Blueprints/FirstPersonCharacter.FirstPersonCharacter_C|GetIsInspecting? (Variables|/Game/_ConvergencePoint/Blueprints/HighLevelBP/MyGameManager.MyGameManager_C|GetMyPlayer _my_game_manager))
    (Default|StartScan (Variables|Default|GetScanner))
    (CallFunction|AddMiscObjecttoLogbook)))

(event Collision|EventActorEndOverlap
  (params (OtherActor :type Actor%20Object%20Reference))
  (if (== OtherActor (Game|GetPlayerCharacter 0))
    (CallFunction|EndOverlap OtherActor)
    (CallFunction|RemoveOutline)))

(fn ConstructionScript
  (bind _miscobjectmesh (Variables|Default|GetMiscObjectMesh))
  (|CallParentFunction)
  (Components|StaticMesh|SetStaticMesh (Variables|Default|GetInteractableMesh) _miscobjectmesh)
  (Components|StaticMesh|SetStaticMesh (Variables|Default|GetInspectionMesh) _miscobjectmesh)
  (bind _asbp_scanner_base (Utilities|Casting|CastToBP_ScannerBase (Variables|/Script/Engine.ChildActorComponent|GetChildActor (Variables|Default|GetBP_ScannerBase))))
  (Variables|Default|SetScanner _asbp_scanner_base))

(fn AddMiscObjecttoLogbook
  (bind _my_game_manager (CallFunction|GetMyGameManager))
  (Utilities|Array|AddUnique (Variables|/Game/FirstPersonBP/Blueprints/FirstPersonCharacter.FirstPersonCharacter_C|GetInventory (Variables|/Game/_ConvergencePoint/Blueprints/HighLevelBP/MyGameManager.MyGameManager_C|GetMyPlayer _my_game_manager)) (Variables|Default|GetInteractableObjectStruct)))