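; Base scanner actor that shows a laser scan slab sweeping vertically through a box volume.
; The construction script fits the box between two corner vectors, sizes a hidden cube to its footprint and applies a dynamic scan material with laser parameters.
; startScan toggles scanning, setting visibility and material fade, while a timeline scaled to the scan duration drives the cube's height through a float curve.
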(event Custom|Update%20Scan%20Position
  (params (Position%20Alpha :type Float%20%28single-precision%29))
  (bind _box (Variables|Default|GetBox))
  (bind _relativelocation (Variables|/Script/Engine.SceneComponent|GetRelativeLocation _box))
  (bind (_x _y) (Math|Vector|BreakVector _relativelocation))
  ;[1 1 1] Cube movement
  (Transformation|SetRelativeLocation (Variables|Default|GetCube) (Math|Vector|MakeVector _x _y (Math|Float|Lerp (.z (Variables|Default|GetBottom%20Corner)) (.z (Variables|Default|GetTop%20Corner)) Position%20Alpha)) false false))

(event Custom|startScan
  (bind _height_alpha (Variables|Default|GetHeight%20Alpha))
  (bind _scan_mid (Variables|Default|GetScan%20MID))
  (bind _cube (Variables|Default|GetCube))
  ;[1 1 1] Restart scan when interaction ends
  (if (Variables|Default|GetIs%20Scanning?)
    (Rendering|SetVisibility _cube false false)
    (Variables|Default|SetIs%20Scanning? false)
    (Rendering|Material|SetScalarParameterValue _scan_mid "Fade Offset" 0.0 :!class /Script/Engine.MaterialInstanceDynamic)
    (Audio|Components|Audio|Stop (Variables|Default|GetHeight%20Alpha))
    (else
      (Rendering|SetVisibility _cube true false)
      (Variables|Default|SetIs%20Scanning? true)
      (Rendering|Material|SetScalarParameterValue _scan_mid "Fade Offset" (Variables|Default|GetFate%20Offset) :!class /Script/Engine.MaterialInstanceDynamic)
      ;[1 1 1] Adjust playrate
      (Components|Timeline|SetPlayRate _height_alpha (/ 1.0 (Variables|Default|GetScan%20Duration)))
      (Components|Timeline|PlayfromStart _height_alpha)
      ;[1 1 1] Play timelime to make scane effect move up and down
      (bind _alpha (Timeline|Height%20Alpha Play)
        (:Update
          (CallFunction|UpdateScanPosition (Math|Curves|GetFloatValue (Variables|Default|GetScan%20height%20interpolation%20curve) _alpha)))))))

(event EventBeginPlay)

(event Collision|EventActorBeginOverlap
  (params (OtherActor :type Actor%20Object%20Reference)))

(event EventTick
  (params (DeltaSeconds :type Float%20%28single-precision%29)))

(fn ConstructionScript
  (bind _top_corner (Variables|Default|GetTop%20Corner))
  (bind _cube (Variables|Default|GetCube))
  (bind _bottom_corner (Variables|Default|GetBottom%20Corner))
  (bind _box (Variables|Default|GetBox))
  (bind _returnvalue (Components|Box|GetScaledBoxExtent _box))
  (bind _returnvalue_2 (* _returnvalue 2.0))
  (bind _my_game_manager (CallFunction|GetMyGameManager))
  (Variables|Default|SetGameManager _my_game_manager)
  (Utilities|FlowControl|Sequence
    (:then_0
      ;[1 1 1] Scale box collision to fit corners
      (Transformation|SetRelativeLocation (Variables|Default|GetBox) (* (+ _top_corner _bottom_corner) 0.5) false false)
      (Components|Box|SetBoxExtent (Variables|Default|GetBox) (* (- _top_corner _bottom_corner) 0.5) false))
    (:then_1
      ;[1 1 1] Create dynamic material
      (bind _returnvalue_3 (Rendering|Material|CreateDynamicMaterialInstance (Variables|Default|GetScan%20Material%20Parent) "None" :!class /Script/Engine.KismetMaterialLibrary))
      (bind _output_get (Variables|Default|SetScan%20MID _returnvalue_3))
      (Rendering|Material|SetScalarParameterValue _output_get "Laser Contact Distance" (Variables|Default|GetLaser%20Contact%20Distance) :!class /Script/Engine.MaterialInstanceDynamic)
      (Rendering|Material|SetScalarParameterValue _output_get "Laser Contact Glow" (Variables|Default|GetLaser%20Contact%20Glow) :!class /Script/Engine.MaterialInstanceDynamic)
      (Rendering|Material|SetScalarParameterValue _output_get "Laser Glow" (Variables|Default|GetLaser%20Glow) :!class /Script/Engine.MaterialInstanceDynamic)
      ;[1 1 1] Scale cube mesh accordingly
      (Transformation|SetRelativeScale3D (Variables|Default|GetCube) (* (Math|Vector|MakeVector (.x _returnvalue_2) (.y _returnvalue_2) (Variables|Default|GetCube%20height)) 0.01))
      ;[1 1 1] Position cube mesh to center of box
      (Transformation|SetRelativeLocation (Variables|Default|GetCube) (Variables|/Script/Engine.SceneComponent|GetRelativeLocation (Variables|Default|GetBox)) false false)
      ;[1 1 1] Apply Scan material
      (Rendering|Material|SetMaterial _cube 0 (Variables|Default|GetScan%20MID))
      ;[1 1 1] Start invisble
      (Rendering|SetVisibility _cube false false))))