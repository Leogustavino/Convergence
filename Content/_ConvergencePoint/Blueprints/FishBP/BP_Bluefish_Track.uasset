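; BP_Bluefish_Track moves a scene component along a spline, evidently as the swim path of a bluefish.
; On BeginPlay a timeline maps its track value to distance along the spline and updates the component's transform, keeping its scale.
; Location is sampled in world space, but rotation is sampled in spline-local space and applied as a world rotation.
; The timeline replays from the start when finished, looping the motion endlessly.
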(event EventBeginPlay
  (bind _spline (Variables|Default|GetSpline))
  (bind _scene (Variables|Default|GetScene))
  (bind _newtrack_0 (Timeline|Timeline_0 Play)
    (:Update
      (Transformation|SetWorldTransform _scene (Math|Transform|MakeTransform (Spline|GetLocationatDistanceAlongSpline _spline (* (Spline|GetSplineLength _spline) _newtrack_0) "World") (Spline|GetRotationatDistanceAlongSpline _spline (* (Spline|GetSplineLength _spline) _newtrack_0) "Local") (Transformation|GetWorldScale _scene)) false false))
    (:Finished
      (while false
        _)
      (Timeline|Timeline_0 PlayFromStart))))

(fn ConstructionScript)