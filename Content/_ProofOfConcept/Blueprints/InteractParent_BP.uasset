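; Parent Blueprint for interactable objects that the player can inspect up close with dialog and audio.
; Box overlap toggles the interaction prompt through the game manager's widgets.
; Interact toggles inspection: it moves the mesh to the player's inspection point, shows dialog, plays audio and disables movement, then reverses this using the object transform stored on the player.
; Tick keeps the audio cue on the player's mesh.
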(event OnComponentBeginOverlap(BoxCollision)
  (params (OverlappedComponent :type Primitive%20Component%20Object%20Reference) (OtherActor :type Actor%20Object%20Reference) (OtherComp :type Primitive%20Component%20Object%20Reference) (OtherBodyIndex :type Integer) (bFromSweep :type Boolean) (SweepResult :type Hit%20Result%20Structure%20%28by%20ref%29))
  ;[1 1 1] Show Interaction
  (CallFunction|BeginOverlap OtherActor))

(event OnComponentEndOverlap(BoxCollision)
  (params (OverlappedComponent :type Primitive%20Component%20Object%20Reference) (OtherActor :type Actor%20Object%20Reference) (OtherComp :type Primitive%20Component%20Object%20Reference) (OtherBodyIndex :type Integer))
  ;[1 1 1] Hide Interaction
  (CallFunction|EndOverlap OtherActor))

(event EventBeginPlay
  (Variables|Default|SetAudioCue (Variables|Default|GetFire01_Cue)))

(event Collision|EventActorBeginOverlap
  (params (OtherActor :type Actor%20Object%20Reference)))

(event EventTick
  (params (DeltaSeconds :type Float%20%28single-precision%29))
  ;[1 1 1] Audio follow player
  (CallFunction|AudioFollow))

(event EventInteract
  (params (PlayerInteracted :type Actor%20Object%20Reference))
  ;[1 1 1] Player interaction
  (CallFunction|PlayerInteraction PlayerInteracted false))

(fn ConstructionScript)

(fn BeginOverlap
  (params (OverlappingActor :type Actor%20Object%20Reference))
  (bind _my_game_manager (CallFunction|GetMyGameManager))
  (if (== OverlappingActor (Variables|/Game/_ProofOfConcept/Blueprints/MyGameManager.MyGameManager_C|GetMyPlayer _my_game_manager))
    (Widget|SetVisibility (Variables|/Game/_ProofOfConcept/Blueprints/MyGameManager.MyGameManager_C|GetInteractionWidget _my_game_manager) "Visible")))

(fn EndOverlap
  (params (Overlapping%20Actor :type Actor%20Object%20Reference))
  (bind _my_game_manager (CallFunction|GetMyGameManager))
  (if (== Overlapping%20Actor (Variables|/Game/_ProofOfConcept/Blueprints/MyGameManager.MyGameManager_C|GetMyPlayer _my_game_manager))
    (Widget|SetVisibility (Variables|/Game/_ProofOfConcept/Blueprints/MyGameManager.MyGameManager_C|GetInteractionWidget _my_game_manager) "Hidden")))

(fn PlayerInteraction
  (params (PlayerInteracted :type Actor%20Object%20Reference) (IsInpecting? :type Boolean))
  (bind _audiocue (Variables|Default|GetAudioCue))
  (bind _isoverlapping (CallFunction|IsOverlapping (Variables|Default|GetBoxCollision) PlayerInteracted))
  (bind _my_game_manager (CallFunction|GetMyGameManager))
  (if _isoverlapping
    (if (Variables|/Game/FirstPersonBP/Blueprints/FirstPersonCharacter.FirstPersonCharacter_C|GetIsInspecting? (Variables|/Game/_ProofOfConcept/Blueprints/MyGameManager.MyGameManager_C|GetMyPlayer _my_game_manager))
      ;[1 1 1] Stop Audio & Hide Dialog
      (Widget|SetVisibility (Variables|/Game/_ProofOfConcept/Blueprints/MyGameManager.MyGameManager_C|GetDialogWidget _my_game_manager) "Hidden")
      (Audio|Components|Audio|Stop _audiocue)
      ;[1 1 1] Put back the object in original location
      (CallFunction|ReleaseObject)
      ;[1 1 1] Enable movement
      (Pawn|Components|CharacterMovement|SetMovementMode (Variables|/Script/Engine.Character|GetCharacterMovement (Variables|/Game/_ProofOfConcept/Blueprints/MyGameManager.MyGameManager_C|GetMyPlayer _my_game_manager)) "MOVE_Walking" 0)
      (bind _my_game_manager_2 (CallFunction|GetMyGameManager))
      (Variables|/Game/FirstPersonBP/Blueprints/FirstPersonCharacter.FirstPersonCharacter_C|SetIsInspecting? (Variables|/Game/_ProofOfConcept/Blueprints/MyGameManager.MyGameManager_C|GetMyPlayer _my_game_manager_2) false)
      (else
        ;[1 1 1] Play Audio & Dialog
        (Widget|SetVisibility (Variables|/Game/_ProofOfConcept/Blueprints/MyGameManager.MyGameManager_C|GetDialogWidget _my_game_manager) "Visible")
        (Audio|Components|Audio|Play _audiocue 0.0)
        ;[1 1 1] Inspect/Move object to front of camera
        (CallFunction|InspectObject)
        ;[1 1 1] Disable Movement
        (Pawn|Components|CharacterMovement|DisableMovement (Variables|/Script/Engine.Character|GetCharacterMovement (Variables|/Game/_ProofOfConcept/Blueprints/MyGameManager.MyGameManager_C|GetMyPlayer _my_game_manager)))
        (bind _my_game_manager_3 (CallFunction|GetMyGameManager))
        (Variables|/Game/FirstPersonBP/Blueprints/FirstPersonCharacter.FirstPersonCharacter_C|SetIsInspecting? (Variables|/Game/_ProofOfConcept/Blueprints/MyGameManager.MyGameManager_C|GetMyPlayer _my_game_manager_3) true)))))

(fn AudioFollow
  (bind _my_game_manager (CallFunction|GetMyGameManager))
  (Transformation|SetWorldTransform (Variables|Default|GetAudioCue) (Transformation|GetWorldTransform (Variables|/Script/Engine.Character|GetMesh (Variables|/Game/_ProofOfConcept/Blueprints/MyGameManager.MyGameManager_C|GetMyPlayer _my_game_manager))) false false))

(fn InspectObject
  ;[1 1 1] Move inspectable object in front of camera
  (bind _my_game_manager (CallFunction|GetMyGameManager))
  (Transformation|SetWorldLocation (Variables|Default|GetInspectionMesh) (Transformation|GetWorldLocation (Variables|/Game/FirstPersonBP/Blueprints/FirstPersonCharacter.FirstPersonCharacter_C|GetInspectionLocation (Variables|/Game/_ProofOfConcept/Blueprints/MyGameManager.MyGameManager_C|GetMyPlayer _my_game_manager))) false false))

(fn ReleaseObject
  (bind _my_game_manager (CallFunction|GetMyGameManager))
  (Transformation|SetWorldLocation (Variables|/Game/FirstPersonBP/Blueprints/FirstPersonCharacter.FirstPersonCharacter_C|GetInspectionObject (Variables|/Game/_ProofOfConcept/Blueprints/MyGameManager.MyGameManager_C|GetMyPlayer _my_game_manager)) (Variables|/Game/FirstPersonBP/Blueprints/FirstPersonCharacter.FirstPersonCharacter_C|GetInspectionObjectLocation (Variables|/Game/_ProofOfConcept/Blueprints/MyGameManager.MyGameManager_C|GetMyPlayer _my_game_manager)) false false)
  (Transformation|SetWorldRotation (Variables|/Game/FirstPersonBP/Blueprints/FirstPersonCharacter.FirstPersonCharacter_C|GetInspectionObject (Variables|/Game/_ProofOfConcept/Blueprints/MyGameManager.MyGameManager_C|GetMyPlayer _my_game_manager)) (Variables|/Game/FirstPersonBP/Blueprints/FirstPersonCharacter.FirstPersonCharacter_C|GetInspectionObjectRotation (Variables|/Game/_ProofOfConcept/Blueprints/MyGameManager.MyGameManager_C|GetMyPlayer _my_game_manager)) false false))