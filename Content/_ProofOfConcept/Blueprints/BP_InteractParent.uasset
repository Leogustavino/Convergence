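; Base interactable object the player can inspect up close, with dialog and audio.
; Box overlap toggles the interaction prompt and an outline, built as a runtime mesh copy with a dynamic material.
; Interact starts the Scanner and, while overlapping, toggles inspection: placing InspectionMesh before the camera, disabling movement and playing dialog audio, or reversing this.
; Shared widgets and player state come through the game manager; Tick keeps audio on the player.
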(event OnComponentBeginOverlap(BoxCollision)
  (params (OverlappedComponent :type Primitive%20Component%20Object%20Reference) (OtherActor :type Actor%20Object%20Reference) (OtherComp :type Primitive%20Component%20Object%20Reference) (OtherBodyIndex :type Integer) (bFromSweep :type Boolean) (SweepResult :type Hit%20Result%20Structure%20%28by%20ref%29))
  ;[1 1 1] Show Interaction
  (if (== OtherActor (Game|GetPlayerCharacter 0))
    (CallFunction|BeginOverlap OtherActor)
    (CallFunction|DrawOutline)))

(event OnComponentEndOverlap(BoxCollision)
  (params (OverlappedComponent :type Primitive%20Component%20Object%20Reference) (OtherActor :type Actor%20Object%20Reference) (OtherComp :type Primitive%20Component%20Object%20Reference) (OtherBodyIndex :type Integer))
  ;[1 1 1] Hide Interaction
  (if (== OtherActor (Game|GetPlayerCharacter 0))
    (CallFunction|EndOverlap OtherActor)
    (CallFunction|RemoveOutline)))

(event EventBeginPlay
  (Variables|Default|SetAudioCue (Variables|Default|GetFire01_Cue)))

(event Collision|EventActorBeginOverlap
  (params (OtherActor :type Actor%20Object%20Reference)))

(event EventTick
  (params (DeltaSeconds :type Float%20%28single-precision%29))
  ;[1 1 1] Audio follow player
  (CallFunction|AudioFollow))

(event EventInteract
  (params (PlayerInteracted :type Actor%20Object%20Reference))
  ;[1 1 1] Player interaction
  (CallFunction|PlayerInteraction PlayerInteracted)
  (Default|StartScan (Variables|Default|GetScanner)))

(fn ConstructionScript)

(fn BeginOverlap
  (params (OverlappingActor :type Actor%20Object%20Reference))
  (bind _my_game_manager (CallFunction|GetMyGameManager))
  (if (== OverlappingActor (Variables|/Game/_ProofOfConcept/Blueprints/MyGameManager.MyGameManager_C|GetMyPlayer _my_game_manager))
    (Widget|SetVisibility (Variables|/Game/_ProofOfConcept/Blueprints/MyGameManager.MyGameManager_C|GetInteractionWidget _my_game_manager) "Visible")))

(fn EndOverlap
  (params (Overlapping%20Actor :type Actor%20Object%20Reference))
  (bind _my_game_manager (CallFunction|GetMyGameManager))
  (if (== Overlapping%20Actor (Variables|/Game/_ProofOfConcept/Blueprints/MyGameManager.MyGameManager_C|GetMyPlayer _my_game_manager))
    (Widget|SetVisibility (Variables|/Game/_ProofOfConcept/Blueprints/MyGameManager.MyGameManager_C|GetInteractionWidget _my_game_manager) "Hidden")))

(fn PlayerInteraction
  (params (PlayerInteracted :type Actor%20Object%20Reference))
  (bind _audiocue (Variables|Default|GetAudioCue))
  (bind _isoverlapping (CallFunction|IsOverlapping (Variables|Default|GetBoxCollision) PlayerInteracted))
  (if _isoverlapping
    (bind _my_game_manager (CallFunction|GetMyGameManager))
    (Variables|/Game/_ProofOfConcept/Blueprints/MyGameManager.MyGameManager_C|SetInteractableObject _my_game_manager self)
    (if (Variables|/Game/FirstPersonBP/Blueprints/FirstPersonCharacter.FirstPersonCharacter_C|GetIsInspecting? (Variables|/Game/_ProofOfConcept/Blueprints/MyGameManager.MyGameManager_C|GetMyPlayer _my_game_manager))
      ;[1 1 1] Stop Audio & Hide Dialog
      (Widget|SetVisibility (Variables|/Game/_ProofOfConcept/Blueprints/MyGameManager.MyGameManager_C|GetDialogWidget _my_game_manager) "Hidden")
      (Audio|Components|Audio|Stop _audiocue)
      ;[1 1 1] Put back the object in original location
      (CallFunction|ReleaseObject)
      ;[1 1 1] Enable movement
      (Pawn|Components|CharacterMovement|SetMovementMode (Variables|/Script/Engine.Character|GetCharacterMovement (Variables|/Game/_ProofOfConcept/Blueprints/MyGameManager.MyGameManager_C|GetMyPlayer _my_game_manager)) "MOVE_Walking" 0)
      (Transformation|SetWorldScale3D (Variables|Default|GetInspectionMesh) "0, 0, 0")
      (bind _my_game_manager_2 (CallFunction|GetMyGameManager))
      (Variables|/Game/FirstPersonBP/Blueprints/FirstPersonCharacter.FirstPersonCharacter_C|SetIsInspecting? (Variables|/Game/_ProofOfConcept/Blueprints/MyGameManager.MyGameManager_C|GetMyPlayer _my_game_manager_2) false)
      (else
        ;[1 1 1] Play Audio & Dialog
        (Widget|SetVisibility (Variables|/Game/_ProofOfConcept/Blueprints/MyGameManager.MyGameManager_C|GetDialogWidget _my_game_manager) "Visible")
        (Audio|Components|Audio|Play _audiocue 0.0)
        ;[1 1 1] Inspect/Move object to front of camera
        (CallFunction|InspectObject)
        ;[1 1 1] Disable Movement
        (Pawn|Components|CharacterMovement|DisableMovement (Variables|/Script/Engine.Character|GetCharacterMovement (Variables|/Game/_ProofOfConcept/Blueprints/MyGameManager.MyGameManager_C|GetMyPlayer _my_game_manager)))
        (Transformation|SetWorldScale3D (Variables|Default|GetInspectionMesh) (Variables|Default|GetScale))
        (bind _my_game_manager_3 (CallFunction|GetMyGameManager))
        (Variables|/Game/FirstPersonBP/Blueprints/FirstPersonCharacter.FirstPersonCharacter_C|SetIsInspecting? (Variables|/Game/_ProofOfConcept/Blueprints/MyGameManager.MyGameManager_C|GetMyPlayer _my_game_manager_3) true)
        (CallFunction|SetObjectSelection)))))

(fn AudioFollow
  (bind _my_game_manager (CallFunction|GetMyGameManager))
  (Transformation|SetWorldTransform (Variables|Default|GetAudioCue) (Transformation|GetWorldTransform (Variables|/Script/Engine.Character|GetMesh (Variables|/Game/_ProofOfConcept/Blueprints/MyGameManager.MyGameManager_C|GetMyPlayer _my_game_manager))) false false))

(fn InspectObject
  (bind _inspectionmesh (Variables|Default|GetInspectionMesh))
  ;[1 1 1] Move inspectable object in front of camera
  (bind _my_game_manager (CallFunction|GetMyGameManager))
  (Transformation|SetWorldLocation _inspectionmesh (Transformation|GetWorldLocation (Variables|/Game/FirstPersonBP/Blueprints/FirstPersonCharacter.FirstPersonCharacter_C|GetInspectionLocation (Variables|/Game/_ProofOfConcept/Blueprints/MyGameManager.MyGameManager_C|GetMyPlayer _my_game_manager))) false false)
  (Transformation|SetWorldRotation _inspectionmesh (Math|Rotator|FindLookatRotation (Transformation|GetWorldLocation (Variables|/Game/FirstPersonBP/Blueprints/FirstPersonCharacter.FirstPersonCharacter_C|GetInspectionLocation (Variables|/Game/_ProofOfConcept/Blueprints/MyGameManager.MyGameManager_C|GetMyPlayer _my_game_manager))) (Transformation|GetWorldLocation (Variables|/Game/FirstPersonBP/Blueprints/FirstPersonCharacter.FirstPersonCharacter_C|GetFirstPersonCamera (Variables|/Game/_ProofOfConcept/Blueprints/MyGameManager.MyGameManager_C|GetMyPlayer _my_game_manager)))) false false))

(fn ReleaseObject
  (bind _my_game_manager (CallFunction|GetMyGameManager))
  (Transformation|SetWorldLocation (Variables|/Game/FirstPersonBP/Blueprints/FirstPersonCharacter.FirstPersonCharacter_C|GetInspectionObject (Variables|/Game/_ProofOfConcept/Blueprints/MyGameManager.MyGameManager_C|GetMyPlayer _my_game_manager)) (Variables|/Game/FirstPersonBP/Blueprints/FirstPersonCharacter.FirstPersonCharacter_C|GetInspectionObjectLocation (Variables|/Game/_ProofOfConcept/Blueprints/MyGameManager.MyGameManager_C|GetMyPlayer _my_game_manager)) false false)
  (Transformation|SetWorldRotation (Variables|/Game/FirstPersonBP/Blueprints/FirstPersonCharacter.FirstPersonCharacter_C|GetInspectionObject (Variables|/Game/_ProofOfConcept/Blueprints/MyGameManager.MyGameManager_C|GetMyPlayer _my_game_manager)) (Variables|/Game/FirstPersonBP/Blueprints/FirstPersonCharacter.FirstPersonCharacter_C|GetInspectionObjectRotation (Variables|/Game/_ProofOfConcept/Blueprints/MyGameManager.MyGameManager_C|GetMyPlayer _my_game_manager)) false false))

(fn DrawOutline
  (bind _interactablemesh (Variables|Default|GetInteractableMesh))
  (if (not (Variables|Default|GetHas%20Outline?))
    (bind _returnvalue (AddComponent|AddStaticMeshComponent true (Transformation|GetWorldTransform _interactablemesh)))
    (bind _output_get (Variables|Default|SetOutlineMesh _returnvalue))
    (Components|StaticMesh|SetStaticMesh _output_get (Variables|/Script/Engine.StaticMeshComponent|GetStaticMesh _interactablemesh))
    (bind _returnvalue_2 (Rendering|Material|CreateDynamicMaterialInstance _output_get 0 "/Game/_ProofOfConcept/Material/M_Outline_Inst.M_Outline_Inst" "None" :!class /Script/Engine.PrimitiveComponent))
    (Rendering|Material|SetVectorParameterValue _returnvalue_2 "Color" (Variables|Default|GetColor) :!class /Script/Engine.MaterialInstanceDynamic)
    (Rendering|Material|SetScalarParameterValue _returnvalue_2 "None" (Variables|Default|GetScaleOutline) :!class /Script/Engine.MaterialInstanceDynamic)
    (Variables|Default|SetHas%20Outline? true)))

(fn RemoveOutline
  (bind _outlinemesh (Variables|Default|GetOutlineMesh))
  (Utilities|IsValid _outlinemesh
    (:Is%20Valid
      (Components|DestroyComponent _outlinemesh)
      (Variables|Default|SetHas%20Outline? false))))