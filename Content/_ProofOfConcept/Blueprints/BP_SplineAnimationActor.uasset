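; Proof-of-concept actor that moves a static mesh along a spline when the player character enters its trigger box.
; The box overlap plays a timeline whose alpha, multiplied by the spline length, gives a distance along the spline.
; Each update sets the mesh's world location and rotation from the spline at that distance, keeping its current scale.
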(event OnComponentBeginOverlap(Box)
  (params (OverlappedComponent :type Primitive%20Component%20Object%20Reference) (OtherActor :type Actor%20Object%20Reference) (OtherComp :type Primitive%20Component%20Object%20Reference) (OtherBodyIndex :type Integer) (bFromSweep :type Boolean) (SweepResult :type Hit%20Result%20Structure%20%28by%20ref%29))
  (bind _spline (Variables|Default|GetSpline))
  (if (== OtherActor (Game|GetPlayerCharacter 0))
    (bind _animation_alpha (Timeline|SplineAnimation Play)
      (:Update
        (Transformation|SetWorldTransform (Variables|Default|GetStaticMesh) (Math|Transform|MakeTransform (Spline|GetLocationatDistanceAlongSpline _spline (* (Spline|GetSplineLength _spline) _animation_alpha) "World") (Spline|GetRotationatDistanceAlongSpline _spline (* (Spline|GetSplineLength _spline) _animation_alpha) "World") (Transformation|GetWorldScale (Variables|Default|GetStaticMesh))) false false)))))

(event EventBeginPlay)

(event Collision|EventActorBeginOverlap
  (params (OtherActor :type Actor%20Object%20Reference)))

(event EventTick
  (params (DeltaSeconds :type Float%20%28single-precision%29)))

(fn ConstructionScript)